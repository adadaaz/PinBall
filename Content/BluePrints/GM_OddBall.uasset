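; Game mode for Oddball, a timed capture-ball match built on a parent game mode.
; On BeginPlay it creates players, resets the timer and BallMG state, attaches the HUD, spawns the capture ball, and finds the item spawner and store.
; Tick only counts the timer down; EndGame pauses play and shows the game-over widget with UI-only input.
; PurchaseItem and SkipItem are empty stubs.
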(event Custom|GetItemSpawner
  (bind _outactors (Actor|GetAllActorsOfClass "/Game/BluePrints/BP_RandomItemSpawner.BP_RandomItemSpawner_C"))
  (Variables|Default|SetRndSpawner (Utilities|Array|Get(acopy) _outactors)))

(event EventStartGame
  (CallFunction|CreatePlayers)
  (CallFunction|InitializeVars)
  (CallFunction|AttachHUD))

(event EventCreatePlayers
  (|CallParentFunction)
  (Variables|/Game/BluePrints/BP_BallManager.BP_BallManager_C|SetOddBallEnd (Variables|Default|GetBallMG) false))

(event EventBeginPlay
  (CallFunction|StartGame)
  (Default|CreateCaptureBall (Variables|Default|GetBallMG))
  (CallFunction|GetItemSpawner)
  (CallFunction|GetStore)
  (Utilities|Array|Resize (Variables|/Game/BluePrints/BP_BallManager.BP_BallManager_C|GetSortedTestBall (Variables|Default|GetBallMG)) 4))

(event EventTick
  (params (DeltaSeconds :type Float%20%28single-precision%29))
  (Variables|Default|SetGamePlayTime (- (Variables|Default|GetGamePlayTime) DeltaSeconds)))

(event EventEndGame
  (bind _returnvalue (Game|GetPlayerController 0))
  (Variables|Default|SetGamePlayTime 0.0)
  (Game|SetGamePaused true)
  (Viewport|RemoveAllWidgets)
  (Variables|/Script/Engine.PlayerController|SetbShowMouseCursor _returnvalue true)
  (bind _returnvalue_2 (UserInterface|CreateWidget "/Game/UI/OddballGameover.OddballGameover_C" _returnvalue))
  (UserInterface|Viewport|AddtoViewport _returnvalue_2 0)
  (Input|SetInputModeUIOnly _returnvalue _returnvalue_2 "DoNotLock"))

(event EventPurchaseItem
  (params (controllerID :type Integer)))

(event EventSkipItem
  (params (controllerID :type Integer)))

(fn ConstructionScript
  (|CallParentFunction))

(fn InitializeVars
  (Variables|Default|SetGamePlayTime (Variables|Default|GetOverallGameTime))
  (Variables|/Game/BluePrints/BP_BallManager.BP_BallManager_C|SetMode (Variables|Default|GetBallMG) 1))

(fn AttachHUD
  (bind _returnvalue (Game|GetPlayerController 0))
  (Viewport|RemoveAllWidgets)
  (bind _returnvalue_2 (UserInterface|CreateWidget "/Game/UI/OddBallHUD.OddBallHUD_C" _returnvalue))
  (UserInterface|Viewport|AddtoViewport _returnvalue_2 0)
  (Input|SetInputModeGameOnly _returnvalue))