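; BP_Flipper is an actor with a Flipper component that rotates between a start and an end rotation, like a pinball flipper.
; Flip and Flop events use MoveComponentTo to rotate it to opposite poses over FlipTime.
; An IsFlip flag swaps which rotation each event targets, and the construction script uses it to set the resting rotation.
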(event Custom|Flip
  ;[1 1 1] Flip
  (if (Variables|Default|GetIsFlip)
    (Components|MoveComponentTo (Variables|Default|GetFlipper) "0, 0, 0" (Variables|Default|GetStartRot) false false (Variables|Default|GetFlipTime) false)
    (else
      (Components|MoveComponentTo (Variables|Default|GetFlipper) "0, 0, 0" (Variables|Default|GetEndRot) false false (Variables|Default|GetFlipTime) false))))

(event Custom|Flop
  ;[1 1 1] Flop
  (if (Variables|Default|GetIsFlip)
    (Components|MoveComponentTo (Variables|Default|GetFlipper) "0, 0, 0" (Variables|Default|GetEndRot) false false (Variables|Default|GetFlipTime) false)
    (else
      (Components|MoveComponentTo (Variables|Default|GetFlipper) "0, 0, 0" (Variables|Default|GetStartRot) false false (Variables|Default|GetFlipTime) false))))

(fn ConstructionScript
  (bind _flipper (Variables|Default|GetFlipper))
  ;[1 1 1] Set starting position
  (if (Variables|Default|GetIsFlip)
    (Transformation|SetRelativeRotation _flipper (Variables|Default|GetEndRot) false false)
    (else
      (Transformation|SetRelativeRotation _flipper (Variables|Default|GetStartRot) false false))))