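; BP_TestBall is a physics-driven player ball prototype for up to four players, coloured by controller ID.
; Input axes push the ball with forces, and hitting another ball applies damage, though damage handling is still a stub.
; Tick maps BallType to a status, pushes the ball down above a height limit and prints health and lives, leaving the speed clamp off.
; Respawn teleports the ball to spawn, briefly hiding it and disabling input.
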(event Custom|Respawn
  ;[1 1 1] Respawn Event
  (Transformation|SetWorldLocation (Variables|Default|GetBall) (Variables|Default|GetSpawnPosition) false false)
  (Physics|SetPhysicsLinearVelocity (Variables|Default|GetBall) (Math|Vector|MakeVector 0.0 0.0 0.0) false "None")
  ;;[1 1 1] Disapper for 0.5s and re-appear
  (Input|DisableInput (Game|GetPlayerController (Variables|Default|GetCtrlId)))
  (Rendering|SetVisibility (Variables|Default|GetBall) false false)
  (Utilities|FlowControl|Delay (Variables|Default|GetRespawnDelay))
  (Input|EnableInput (Game|GetPlayerController (Variables|Default|GetCtrlId)))
  (Rendering|SetVisibility (Variables|Default|GetBall) true false))

(event EventBeginPlay
  (bind _playerscale (Variables|Default|GetPlayerScale))
  (Utilities|FlowControl|Sequence
    (:then_0
      (CallFunction|InitializeMaterial))
    (:then_1
      (Transformation|SetRelativeScale3D (Variables|Default|GetBall) (Math|Vector|MakeVector _playerscale _playerscale _playerscale)))
    (:then_2
      (Variables|Default|SetCurrentHealth (Variables|Default|GetMaxHealth))
      (Variables|Default|SetCurrentLife (Variables|Default|GetMaxLife))
      (Variables|Default|SetBallType 0))))

(event Game|Damage|EventAnyDamage
  (params (Damage :type Float%20%28single-precision%29) (DamageType :type Damage%20Type%20Object%20Reference) (InstigatedBy :type Controller%20Object%20Reference) (DamageCauser :type Actor%20Object%20Reference)))

(event Collision|EventHit
  (params (MyComp :type Primitive%20Component%20Object%20Reference) (Other :type Actor%20Object%20Reference) (OtherComp :type Primitive%20Component%20Object%20Reference) (bSelfMoved :type Boolean) (HitLocation :type Vector :default "0, 0, 0") (HitNormal :type Vector :default "0, 0, 0") (NormalImpulse :type Vector :default "0, 0, 0") (Hit :type Hit%20Result%20Structure%20%28by%20ref%29))
  (bind _asbp_test_ball (Utilities|Casting|CastToBP_TestBall Other))
  (Game|Damage|ApplyDamage _asbp_test_ball (Variables|Default|GetHitDamage) 0 0))

(event EventTick
  (params (DeltaSeconds :type Float%20%28single-precision%29))
  (CallFunction|StatusCheck)
  (CallFunction|ApplyConstraints false)
  (Development|PrintString (Utilities|String|Append "Health: " (Utilities|String|ToString(Float) (Variables|Default|GetCurrentHealth)) "   Life:" (Utilities|String|ToString(Integer) (Variables|Default|GetCurrentLife)))))

(event Input|AxisEvents|InputAxisMoveForward
  (params (AxisValue :type Float%20%28single-precision%29))
  (bind _playeraccel (Variables|Default|GetPlayerAccel))
  ;[1 1 1] Movement
  (Physics|AddForce (Variables|Default|GetBall) (Math|Vector|MakeVector (* AxisValue _playeraccel) (* (stale Input|AxisEvents|InputAxisMoveRight AxisValue) _playeraccel) 0.0) "None" true))

(event Input|AxisEvents|InputAxisMoveRight
  (params (AxisValue :type Float%20%28single-precision%29))
  (bind _playeraccel (Variables|Default|GetPlayerAccel))
  ;[1 1 1] Movement
  (Physics|AddForce (Variables|Default|GetBall) (Math|Vector|MakeVector (* (stale Input|AxisEvents|InputAxisMoveForward AxisValue) _playeraccel) (* AxisValue _playeraccel) 0.0) "None" true))

(fn ConstructionScript)

(fn InitializeMaterial
  (switch int (Variables|Default|GetCtrlId)
    (:0
      (LocalVariables|SetTempPlayerMI "/Game/Rolling/Materials/MI_PlayerBall1.MI_PlayerBall1"))
    (:1
      (LocalVariables|SetTempPlayerMI "/Game/Rolling/Materials/MI_PlayerBall2.MI_PlayerBall2"))
    (:2
      (LocalVariables|SetTempPlayerMI "/Game/Rolling/Materials/MI_PlayerBall3.MI_PlayerBall3"))
    (:3
      (LocalVariables|SetTempPlayerMI "/Game/Rolling/Materials/MI_PlayerBall4.MI_PlayerBall4")))
  (bind _returnvalue (Rendering|Material|CreateDynamicMaterialInstance (LocalVariables|GetTempPlayerMI) "None" :!class /Script/Engine.KismetMaterialLibrary))
  (Rendering|Material|SetMaterial (Variables|Default|GetBall) 0 _returnvalue))

(fn StatusCheck
  (switch int (Variables|Default|GetBallType)
    (:0
      (Variables|Default|SetBallStatus "NewEnumerator0"))
    (:1
      (Variables|Default|SetBallStatus "NewEnumerator1"))
    (:2
      (Variables|Default|SetBallStatus "NewEnumerator2"))
    (:3
      (Variables|Default|SetBallStatus "NewEnumerator3"))))

(fn ApplyConstraints
  (params (CheckVelocity :type Boolean))
  (bind _returnvalue (Transformation|GetVelocity))
  (bind _maxspeed (Variables|Default|GetMaxSpeed))
  (bind _ball (Variables|Default|GetBall))
  (bind (_x _y) (Math|Vector|BreakVector _returnvalue))
  (bind (_x_2 _y_2) (Math|Vector|BreakVector _returnvalue))
  (bind _returnvalue_2 (Math|Vector|MakeVector _x _y 0.0))
  (bind _returnvalue_3 (Math|Vector|Normalize _returnvalue_2))
  (bind _returnvalue_4 (* _returnvalue_3 _maxspeed))
  ;[1 1 1] Height Constraints
  (LocalVariables|SetCheckSpeed CheckVelocity)
  (if (> (.z (Transformation|GetWorldLocation _ball)) (Variables|Default|GetMaxBallHeight))
    (Physics|AddForce _ball "0, 0,-100.000000" "None" true))
  (if (LocalVariables|GetCheckSpeed)
    ;[1 1 1] Speed Constraints
    (if (> (+ (Math|Float|Square _x_2) (Math|Float|Square _y_2)) (Math|Float|Square (Variables|Default|GetMaxSpeed)))
      (Physics|SetPhysicsLinearVelocity (Variables|Default|GetBall) (Math|Vector|MakeVector (.x _returnvalue_4) (.y _returnvalue_4) 0.0) false "None")
      (return))
    (else
      (return))))

(fn TakeDamage
  (params (DMG :type Float%20%28single-precision%29))
  (if (Utilities|Enum|Equal(Enum) (Variables|Default|GetBallStatus) "NewEnumerator0")
    _))