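; BP_LevelSelect manages the front-end menus, swapping between main menu and level select widgets and opening chosen levels.
; On BeginPlay it creates the MainMenu widget for the PC_Ball controller, shows the cursor and sets UI-only input.
; Each menu switch clears all widgets first; DisplayMainMenu re-adds the stored main menu instead of recreating it.
; GoToLevel opens a level by name and leaves its index input unused.
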(event Custom|Construct%20MainMenu
  (bind _returnvalue (Game|GetPlayerController 0))
  (Viewport|RemoveAllWidgets)
  (bind _aspc_ball (Utilities|Casting|CastToPC_Ball (Game|GetPlayerController 0)))
  (bind _returnvalue_2 (UserInterface|CreateWidget "/Game/UI/MainMenu.MainMenu_C" _aspc_ball))
  (Variables|Default|SetWG_MainMenu _returnvalue_2)
  (UserInterface|Viewport|AddtoViewport _returnvalue_2 0)
  (Input|SetInputModeUIOnly _returnvalue _returnvalue_2 "DoNotLock")
  (Variables|/Script/Engine.PlayerController|SetbShowMouseCursor _returnvalue true))

(event Custom|Construct%20LevelSelectMenu
  (Viewport|RemoveAllWidgets)
  (bind _aspc_ball (Utilities|Casting|CastToPC_Ball (Game|GetPlayerController 0)))
  (bind _returnvalue (UserInterface|CreateWidget "/Game/UI/Level/LevelSelect.LevelSelect_C" _aspc_ball))
  (Variables|Default|SetWG_SelectMenu _returnvalue)
  (UserInterface|Viewport|AddtoViewport _returnvalue 0))

(event EventBeginPlay
  (CallFunction|ConstructMainMenu))

(fn ConstructionScript)

(fn GotoLevel
  (params (LevelIndex :type Integer) (LevelName :type Name))
  (Game|OpenLevel(byName) LevelName))

(fn DisplayMainMenu
  (Viewport|RemoveAllWidgets)
  (UserInterface|Viewport|AddtoViewport (Variables|Default|GetWG_MainMenu) 0))