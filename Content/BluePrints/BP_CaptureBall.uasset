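; BP_CaptureBall is a ball that latches onto the first BP_TestBall it hits and follows it.
; On that hit it stores an offset built from the hit location, sets the ball's HasDeadWeight flag and ignores PhysicsBody collisions.
; While that flag holds, Tick disables physics, zeroes velocity and moves the actor to the ball's XY plus the offset, with Z fixed to the offset's Z.
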(event EventBeginPlay)

(event Collision|EventActorBeginOverlap
  (params (OtherActor :type Actor%20Object%20Reference)))

(event EventTick
  (params (DeltaSeconds :type Float%20%28single-precision%29))
  (bind _lasthitball (Variables|Default|GetLastHitBall))
  (bind _hitoffset (Variables|Default|GethitOffSet))
  (bind _lasthitball_2 (Variables|Default|GetLastHitBall))
  (bind _returnvalue (Transformation|GetActorLocation _lasthitball))
  (Utilities|IsValid _lasthitball_2
    (:Is%20Valid
      (if (Variables|/Game/BluePrints/BP_TestBall.BP_TestBall_C|GethasDeadWeight _lasthitball_2)
        (Physics|SetSimulatePhysics (Variables|Default|GetCaptureBall) false)
        (Transformation|SetActorLocation (Math|Vector|MakeVector (+ (.x _returnvalue) (.x _hitoffset)) (+ (.y _returnvalue) (.y _hitoffset)) (.z _hitoffset)) false false)
        (Physics|SetPhysicsLinearVelocity (Variables|Default|GetCaptureBall) "0, 0, 0" false "None")))))

(event Collision|EventHit
  (params (MyComp :type Primitive%20Component%20Object%20Reference) (Other :type Actor%20Object%20Reference) (OtherComp :type Primitive%20Component%20Object%20Reference) (bSelfMoved :type Boolean) (HitLocation :type Vector :default "0, 0, 0") (HitNormal :type Vector :default "0, 0, 0") (NormalImpulse :type Vector :default "0, 0, 0") (Hit :type Hit%20Result%20Structure%20%28by%20ref%29))
  (bind (_asbp_test_ball _bsuccess) (Utilities|Casting|CastToBP_TestBall Other))
  (if (and _bsuccess (not (Variables|Default|Getcaptured)))
    (Variables|Default|SethitOffSet (+ HitLocation "200.000000,200.000000,0.000000"))
    (bind _output_get (Variables|Default|SetLastHitBall _asbp_test_ball))
    (Variables|/Game/BluePrints/BP_TestBall.BP_TestBall_C|SethasDeadWeight _output_get true)
    (Variables|Default|Setcaptured true)
    (Collision|SetCollisionResponsetoChannel (Variables|Default|GetCaptureBall) "ECC_PhysicsBody" "ECR_Ignore")))

(fn ConstructionScript)