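; BP_Timer is a countdown timer actor that tracks whether a set duration is still running.
; SetTargetTime stores the duration and real-time start, then sets IsTiming, which Tick clears once the elapsed real time reaches the target.
; Expiry fires no event in this graph, it only clears the flag.
; A separate GetDelay event waits a given delay and prints "Time Up", independent of that countdown.
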(event Custom|GetDelay
  (params (Delays :type Float%20%28single-precision%29))
  (Utilities|FlowControl|Delay Delays)
  (Development|PrintString "Time Up"))

(event EventBeginPlay)

(event Collision|EventActorBeginOverlap
  (params (OtherActor :type Actor%20Object%20Reference)))

(event EventTick
  (params (DeltaSeconds :type Float%20%28single-precision%29))
  (if (Variables|Default|GetIsTiming)
    (if (<= (- (Variables|Default|GetTargetTimer) (- (Utilities|Time|GetRealTimeSeconds) (Variables|Default|GetStartTime))) 5e-06)
      (Variables|Default|SetIsTiming false))))

(fn ConstructionScript)

(fn SetTargetTime
  (params (TargetTime :type Float%20%28single-precision%29))
  (Variables|Default|SetTargetTimer TargetTime)
  (Variables|Default|SetIsTiming true)
  (Variables|Default|SetStartTime (Utilities|Time|GetRealTimeSeconds)))