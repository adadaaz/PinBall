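; Player-controlled pinball for up to four players, with a ball material chosen by controller ID.
; Input drives the ball with physics forces, and Tick caps planar speed except during a short dash.
; In ball collisions the faster one knocks the other along its heading and briefly disables its input, as do flipper hits.
; It also handles scoring, respawn at BP_Spawn with temporary collision immunity, and a placeholder pickup.
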(event OnComponentBeginOverlap(Ball)
  (params (OverlappedComponent :type Primitive%20Component%20Object%20Reference) (OtherActor :type Actor%20Object%20Reference) (OtherComp :type Primitive%20Component%20Object%20Reference) (OtherBodyIndex :type Integer) (bFromSweep :type Boolean) (SweepResult :type Hit%20Result%20Structure%20%28by%20ref%29))
  ;[1 1 1] player scores a point
  (bind _asbp_score_point (Utilities|Casting|CastToBP_ScorePoint OtherActor))
  (if (not (Variables|/Game/BluePrints/BP_ScorePoint.BP_ScorePoint_C|GetisHit _asbp_score_point))
    (Variables|Default|SetScore (+ (Variables|Default|GetScore) 100))))

(event Custom|Invulnerable
  ;[1 1 1] Makes the player invulnerable from hitting other players for 3 seconds
  (Collision|SetCollisionResponsetoChannel (Variables|Default|GetBall) "ECC_PhysicsBody" "ECR_Ignore")
  (Development|PrintString "Collison Disabled" true true "(R=1.000000,G=0.019096,B=0.000000,A=1.000000)" 3.0)
  (Utilities|FlowControl|Delay 3.0)
  (Collision|SetCollisionResponsetoChannel (Variables|Default|GetBall) "ECC_PhysicsBody" "ECR_Block")
  (Development|PrintString "Collison Activated" true true "(R=0.000000,G=0.660000,B=1.000000,A=1.000000)" 3.0))

(event Custom|Respawn
  ;[1 1 1] Respawn
  (Transformation|SetWorldLocation (Variables|Default|GetBall) (Variables|Default|GetinitPos) false false)
  (Input|DisableInput (Game|GetPlayerController (Variables|Default|GetCtrlId)))
  (Rendering|SetVisibility (Variables|Default|GetBall) false false)
  (Utilities|FlowControl|Delay 0.5)
  (Input|EnableInput (Game|GetPlayerController (Variables|Default|GetCtrlId)))
  (Rendering|SetVisibility (Variables|Default|GetBall) true false)
  (CallFunction|Invulnerable))

(event Custom|TempDisableInput
  (params (TimeToWait :type Float%20%28single-precision%29))
  (bind _ctrlid (Variables|Default|GetCtrlId))
  (bind _returnvalue (Game|GetPlayerController _ctrlid))
  ;[1 1 1] Temporarily Disable Input
  (Input|DisableInput _returnvalue)
  (Utilities|FlowControl|Delay TimeToWait)
  (Input|EnableInput _returnvalue))

(event EventBeginPlay
  (bind _playerscale (Variables|PlayerVars|GetPlayerScale))
  ;[1 1 1] setting initial position(respawn position) of the ball
  (bind _outactors (Actor|GetAllActorsOfClass "/Game/BluePrints/BP_Spawn.BP_Spawn_C"))
  (bind _ballspawnloc (Default|GetPinballSpawnLocation (Utilities|Array|Get(acopy) _outactors)))
  (Variables|Default|SetinitPos _ballspawnloc)
  (Transformation|SetRelativeScale3D (Variables|Default|GetBall) (Math|Vector|MakeVector _playerscale _playerscale _playerscale)))

(event EventTick
  (params (DeltaSeconds :type Float%20%28single-precision%29))
  (bind _returnvalue (Transformation|GetVelocity))
  (bind (_x _y) (Math|Vector|BreakVector _returnvalue))
  ;[1 1 1] Set current Velocity and Forward Vector and applies the Apply Max Velocity
  (Variables|Default|SetDeltaT DeltaSeconds)
  (Variables|Default|SetForwardVector (Math|Vector|Normalize (Transformation|GetVelocity)))
  (Variables|Default|SetVelocity (Math|Float|Sqrt (+ (Math|Float|Square _x) (Math|Float|Square _y))))
  (if (Variables|Default|GetLimitVelocity)
    (CallFunction|ApplyMaxVelocity)))

(event Collision|EventHit
  (params (MyComp :type Primitive%20Component%20Object%20Reference) (Other :type Actor%20Object%20Reference) (OtherComp :type Primitive%20Component%20Object%20Reference) (bSelfMoved :type Boolean) (HitLocation :type Vector :default "0, 0, 0") (HitNormal :type Vector :default "0, 0, 0") (NormalImpulse :type Vector :default "0, 0, 0") (Hit :type Hit%20Result%20Structure%20%28by%20ref%29))
  ;[1 1 1] Check if ball hits another ball
  (Utilities|FlowControl|Sequence
    (:then_0
      (CallFunction|AddForce Other))
    (:then_1
      (Utilities|Casting|CastToBP_Flipper Other)
      (CallFunction|TempDisableInput (Variables|Default|GetdisableInputWait)))))

(event Input|ActionEvents|InputActionJump
  (params (Key :type Key%20Structure))
  (bind _returnvalue (Transformation|GetVelocity))
  (bind _playerdashspeed (Variables|PlayerVars|GetPlayerDashSpeed))
  (bind _returnvalue_2 (Math|Vector|Normalize _returnvalue))
  (bind _returnvalue_3 (* _returnvalue_2 _playerdashspeed))
  ;[1 1 1] Dash
  (:Pressed
    (Variables|Default|SetLimitVelocity false)
    (Physics|AddForce (Variables|Default|GetBall) (Math|Vector|MakeVector (.x _returnvalue_3) (.y _returnvalue_3) 0.0) "None" true)
    (Utilities|FlowControl|Delay (Variables|Default|GetlimitVelocityWait))
    (Variables|Default|SetLimitVelocity true)))

(event Input|AxisEvents|InputAxisMoveForward
  (params (AxisValue :type Float%20%28single-precision%29))
  (bind _playeraccel (Variables|PlayerVars|GetPlayerAccel))
  ;[1 1 1] Movement
  (Physics|AddForce (Variables|Default|GetBall) (Math|Vector|MakeVector (* _playeraccel AxisValue) (* (stale Input|AxisEvents|InputAxisMoveRight AxisValue) _playeraccel) 0.0) "None" true))

(event Input|AxisEvents|InputAxisMoveRight
  (params (AxisValue :type Float%20%28single-precision%29))
  (bind _playeraccel (Variables|PlayerVars|GetPlayerAccel))
  ;[1 1 1] Movement
  (Physics|AddForce (Variables|Default|GetBall) (Math|Vector|MakeVector (* _playeraccel (stale Input|AxisEvents|InputAxisMoveForward AxisValue)) (* AxisValue _playeraccel) 0.0) "None" true))

(event Input|KeyboardEvents|SpaceBar
  (params (Key :type Key%20Structure))
  ;[1 1 1] PickUp
  (:Pressed
    (if (Variables|Default|GetHasPickUp)
      (Development|PrintString "USE PICK UP")
      (Variables|Default|SetHasPickUp false))))

(fn ConstructionScript
  (bind _ball (Variables|Default|GetBall))
  (Utilities|FlowControl|Sequence
    (:then_0
      (if (== (Variables|Default|GetCtrlId) 0)
        (Rendering|Material|SetMaterial _ball 0 "/Game/Rolling/Materials/MI_PlayerBall1.MI_PlayerBall1")))
    (:then_1
      (if (== (Variables|Default|GetCtrlId) 1)
        (Rendering|Material|SetMaterial _ball 0 "/Game/Rolling/Materials/MI_PlayerBall2.MI_PlayerBall2")))
    (:then_2
      (if (== (Variables|Default|GetCtrlId) 2)
        (Rendering|Material|SetMaterial _ball 0 "/Game/Rolling/Materials/MI_PlayerBall3.MI_PlayerBall3")))
    (:then_3
      (if (== (Variables|Default|GetCtrlId) 3)
        (Rendering|Material|SetMaterial _ball 0 "/Game/Rolling/Materials/MI_PlayerBall4.MI_PlayerBall4")))))

(fn ApplyMaxVelocity
  (bind _returnvalue (Transformation|GetVelocity))
  (bind _maxvelocity (Variables|Default|GetMaxVelocity))
  (bind (_x _y) (Math|Vector|BreakVector _returnvalue))
  (bind (_x_2 _y_2) (Math|Vector|BreakVector _returnvalue))
  (bind _returnvalue_2 (Math|Vector|MakeVector _x _y 0.0))
  (bind _returnvalue_3 (Math|Vector|Normalize _returnvalue_2))
  (bind _returnvalue_4 (* _returnvalue_3 _maxvelocity))
  (if (> (Math|Float|Sqrt (+ (Math|Float|Square _x_2) (Math|Float|Square _y_2))) (Variables|Default|GetMaxVelocity))
    (Physics|SetPhysicsLinearVelocity (Variables|Default|GetBall) (Math|Vector|MakeVector (.x _returnvalue_4) (.y _returnvalue_4) 0.0) false "None")))

(fn AddLiveAbove1500
  (if (>= (Variables|Default|GetScore) 1500)
    (Variables|Default|SetLife (+ (Variables|Default|GetLife) 1))
    (Variables|Default|SetScore 0)))

(fn AddForce
  (params (CollidingActor :type Actor%20Object%20Reference))
  (bind _forwardvector (Variables|Default|GetForwardVector))
  (bind _pinballhitamount (Variables|Default|GetpinballHitAmount))
  (bind _returnvalue (* _forwardvector _pinballhitamount))
  (bind (_x _y) (Math|Vector|BreakVector _returnvalue))
  (bind _asphysics_ball_bp (Utilities|Casting|CastToPinball_BP CollidingActor))
  (CallFunction|SetHitAmount)
  (if (> (Variables|Default|GetVelocity) (Variables|Pinball_BP_C|GetVelocity _asphysics_ball_bp))
    (CallFunction|TempDisableInput _asphysics_ball_bp (Variables|Default|GetdisableInputWait))
    (Physics|SetPhysicsLinearVelocity (Variables|Pinball_BP_C|GetBall _asphysics_ball_bp) (Math|Vector|MakeVector _x _y 0.0) false "None")))

(fn SetHitAmount
  (Variables|Default|SetpinballHitAmount (Variables|Default|GetVelocity))
  (return))