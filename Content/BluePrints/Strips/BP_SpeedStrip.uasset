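; BP_SpeedStrip is a floor strip actor that pushes BP_TestBall along the strip's forward vector, which it refreshes every tick.
; Entering SpeedBox passes force, frequency and direction to the ball's EnterSpeedStrip, and exiting calls LeaveSpeedStrip with a velocity-limit delay.
; On entry it also casts the same actor to PickUp_BumperTime and, if HasInput is set, shows the Ball component and makes it block PhysicsBody.
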(event OnComponentEndOverlap(SpeedBox)
  (params (OverlappedComponent :type Primitive%20Component%20Object%20Reference) (OtherActor :type Actor%20Object%20Reference) (OtherComp :type Primitive%20Component%20Object%20Reference) (OtherBodyIndex :type Integer))
  (bind (_asbp_test_ball _bsuccess) (Utilities|Casting|CastToBP_TestBall OtherActor))
  (if _bsuccess
    (Default|LeaveSpeedStrip _asbp_test_ball (Variables|Default|GetLimitVelocityDelay))))

(event OnComponentBeginOverlap(SpeedBox)
  (params (OverlappedComponent :type Primitive%20Component%20Object%20Reference) (OtherActor :type Actor%20Object%20Reference) (OtherComp :type Primitive%20Component%20Object%20Reference) (OtherBodyIndex :type Integer) (bFromSweep :type Boolean) (SweepResult :type Hit%20Result%20Structure%20%28by%20ref%29))
  (bind (_asbp_test_ball _bsuccess) (Utilities|Casting|CastToBP_TestBall OtherActor))
  (bind _ball (Variables|/Game/BluePrints/BP_TestBall.BP_TestBall_C|GetBall _asbp_test_ball))
  (if _bsuccess
    (Default|EnterSpeedStrip _asbp_test_ball (Variables|Default|GetForce) (Variables|Default|GetAddForceFrequency) (Variables|Default|GetSpeedStripVector))
    (bind _aspick_up_bumper_time (Utilities|Casting|CastToPickUp_BumperTime OtherActor))
    (if (Variables|/Game/BluePrints/PickUps/OddPickups/PickUp_BumperTime.PickUp_BumperTime_C|GetHasInput _aspick_up_bumper_time)
      (Rendering|SetVisibility _ball true false)
      (Collision|SetCollisionResponsetoChannel _ball "ECC_PhysicsBody" "ECR_Block"))))

(event EventTick
  (params (DeltaSeconds :type Float%20%28single-precision%29))
  (Variables|Default|SetSpeedStripVector (Math|Vector|GetForwardVector (Transformation|GetActorRotation))))

(fn ConstructionScript)