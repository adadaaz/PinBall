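; BP_GlueStrip is a glue strip hazard that temporarily slows a Pinball_BP that passes through it.
; On overlap with SlowBox it saves the ball's MaxVelocity and cuts it to 30%.
; When the overlap ends, SlowBox ignores the PhysicsBody channel for five seconds to block re-entry, then restores the saved velocity and overlap response.
; Debug strings print at each stage.
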(event OnComponentBeginOverlap(SlowBox)
  (params (OverlappedComponent :type Primitive%20Component%20Object%20Reference) (OtherActor :type Actor%20Object%20Reference) (OtherComp :type Primitive%20Component%20Object%20Reference) (OtherBodyIndex :type Integer) (bFromSweep :type Boolean) (SweepResult :type Hit%20Result%20Structure%20%28by%20ref%29))
  (Development|PrintString "Glue Strip Activating" true true "(R=0.595707,G=0.567708,B=1.000000,A=1.000000)" 5.0)
  (bind _aspinball_bp (Utilities|Casting|CastToPinball_BP OtherActor))
  (bind _output_get (Variables|Default|SetOldVelocity (Variables|/Game/BluePrints/Pinball_BP.Pinball_BP_C|GetMaxVelocity _aspinball_bp)))
  (Variables|/Game/BluePrints/Pinball_BP.Pinball_BP_C|SetMaxVelocity _aspinball_bp (* _output_get 0.3)))

(event OnComponentEndOverlap(SlowBox)
  (params (OverlappedComponent :type Primitive%20Component%20Object%20Reference) (OtherActor :type Actor%20Object%20Reference) (OtherComp :type Primitive%20Component%20Object%20Reference) (OtherBodyIndex :type Integer))
  (Development|PrintString "Glue Strip Activated" true true "(R=0.064768,G=0.000000,B=1.000000,A=1.000000)" 5.0)
  (bind _aspinball_bp (Utilities|Casting|CastToPinball_BP OtherActor))
  (Development|PrintString "Delay Begins" true true "(R=0.542126,G=0.510417,B=1.000000,A=1.000000)" 5.0)
  (CallFunction|Impenetrable)
  (Utilities|FlowControl|Delay 5.0)
  (Development|PrintString "Delay Done" true true "(R=0.064768,G=0.000000,B=1.000000,A=1.000000)" 5.0)
  (Variables|/Game/BluePrints/Pinball_BP.Pinball_BP_C|SetMaxVelocity _aspinball_bp (Variables|Default|GetOldVelocity))
  (CallFunction|Penetrable))

(event Custom|Impenetrable
  (Collision|SetCollisionResponsetoChannel (Variables|Default|GetSlowBox) "ECC_PhysicsBody" "ECR_Ignore"))

(event Custom|Penetrable
  (Collision|SetCollisionResponsetoChannel (Variables|Default|GetSlowBox) "ECC_PhysicsBody" "ECR_Overlap"))

(event EventBeginPlay)

(event EventTick
  (params (DeltaSeconds :type Float%20%28single-precision%29)))

(fn ConstructionScript)