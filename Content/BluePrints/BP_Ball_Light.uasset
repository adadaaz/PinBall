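; BP_Ball_Light is a light actor that follows an owning test ball and lights it in that player's color.
; On BeginPlay it picks one of four colors from the ball's CtrlID, then each Tick moves to the ball or destroys itself if the ball is invalid.
; DashDamage and Pulse run timelines that animate intensity, then restore the saved value; Pulse skips re-saving it when restarted mid-play.
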(event Custom|DashDamage
  (bind _pointlight (Variables|Default|GetPointLight))
  (Variables|Default|SetReturnIntensity (Variables|/Script/Engine.LightComponentBase|GetIntensity (Variables|Default|GetPointLight)))
  (bind _intensity (Timeline|DashLight PlayFromStart)
    (:Update
      (Rendering|Components|Light|SetIntensity _pointlight _intensity))
    (:Finished
      (Rendering|Components|Light|SetIntensity _pointlight (Variables|Default|GetReturnIntensity)))))

(event Custom|Pulse
  (bind _pointlight (Variables|Default|GetPointLight))
  (if (Audio|Components|Audio|IsPlaying (Variables|Default|GetPulseEffect))
    (bind _intensity (Timeline|PulseEffect PlayFromStart)
      (:Update
        (Rendering|Components|Light|SetIntensity _pointlight _intensity))
      (:Finished
        (Rendering|Components|Light|SetIntensity _pointlight (Variables|Default|GetReturnIntensity))))
    (else
      (Variables|Default|SetReturnIntensity (Variables|/Script/Engine.LightComponentBase|GetIntensity (Variables|Default|GetPointLight)))
      (Timeline|PulseEffect PlayFromStart))))

(event EventTick
  (params (DeltaSeconds :type Float%20%28single-precision%29))
  (bind _owningtestball (Variables|Default|GetowningTestBall))
  (bind _ball (Variables|/Game/BluePrints/BP_TestBall.BP_TestBall_C|GetBall _owningtestball))
  (bind _returnvalue (Transformation|GetWorldLocation _ball))
  (Utilities|IsValid _owningtestball
    (:Is%20Valid
      (Transformation|SetActorLocation (Math|Vector|MakeVector (.x _returnvalue) (.y _returnvalue) (.z _returnvalue)) false false))
    (:Is%20Not%20Valid
      (Actor|DestroyActor))))

(event EventBeginPlay
  (bind _pointlight (Variables|Default|GetPointLight))
  (switch int (Variables|/Game/BluePrints/BP_TestBall.BP_TestBall_C|GetctrlID (Variables|Default|GetowningTestBall))
    (:0
      (Rendering|Components|Light|SetLightColor _pointlight (Variables|Default|GetP1Light) true))
    (:1
      (Rendering|Components|Light|SetLightColor _pointlight (Variables|Default|GetP2Light) true))
    (:2
      (Rendering|Components|Light|SetLightColor _pointlight (Variables|Default|GetP3Light) true))
    (:3
      (Rendering|Components|Light|SetLightColor _pointlight (Variables|Default|GetP4Light) true))))

(fn ConstructionScript)