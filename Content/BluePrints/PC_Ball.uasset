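; PC_Ball is the pinball player controller, handling flipper and pause input and creating a MainMenu widget through its CreatePlayerHUD event.
; On BeginPlay it caches every BP_Flipper in the level, then calls Flip on press and Flop on release for all of them.
; Pause calls PauseGame on GM_PinBall.
; Item purchase and skip inputs are unfinished stubs that only fetch the controller ID.
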(event Custom|CreatePlayerHUD
  ;[1 1 1] Create Player HUD
  (Viewport|RemoveAllWidgets)
  (bind _returnvalue (UserInterface|CreateWidget "/Game/UI/MainMenu.MainMenu_C" self))
  (UserInterface|Viewport|AddtoViewport _returnvalue 0))

(event EventBeginPlay
  ;[1 1 1] Detect Flippers in level
  (CallFunction|DetectFlippers))

(event Input|ActionEvents|InputActionPause
  (params (Key :type Key%20Structure))
  ;[1 1 1] Pause Game
  (:Pressed
    (bind _asgm_pin_ball (Utilities|Casting|CastToGM_PinBall (Game|GetGameMode)))
    (Default|PauseGame _asgm_pin_ball)))

(event Input|ActionEvents|InputActionPurchaseItem
  (params (Key :type Key%20Structure))
  ;[1 1 1] Item Purchase (Y button / Key E)
  (:Pressed
    (bind _returnvalue (Class|GameplayStatics|GetPlayerControllerID self))))

(event Input|ActionEvents|InputActionToggleFlipper
  (params (Key :type Key%20Structure))
  (bind _flippers (Variables|Default|GetFlippers))
  ;[1 1 1] Flip Flippers
  (:Pressed
    (for _array_element _flippers
      (bind _asbp_flipper (Utilities|Casting|CastToBP_Flipper _array_element))
      (Default|Flip _asbp_flipper)))
  (:Released
    (for _array_element_2 _flippers
      (bind _asbp_flipper_2 (Utilities|Casting|CastToBP_Flipper _array_element_2))
      (Default|Flop _asbp_flipper_2))))

(event Input|ActionEvents|InputActionSkipItem
  (params (Key :type Key%20Structure))
  ;[1 1 1] Item Skip (X button / Key Q)
  (:Pressed
    (bind _returnvalue (Class|GameplayStatics|GetPlayerControllerID self))))

(fn ConstructionScript)

(fn DetectFlippers
  (bind _outactors (Actor|GetAllActorsOfClass "/Game/BluePrints/BP_Flipper.BP_Flipper_C"))
  (Variables|Default|SetFlippers _outactors))