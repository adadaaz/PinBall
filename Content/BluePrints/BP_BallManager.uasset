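; Manager actor that spawns and tracks the player balls for local multiplayer pinball matches and checks for game end.
; It creates local players, spawns a BP_TestBall at each BP_Spawn point and has each player controller possess one.
; Tick branches on Mode: OddBall accrues TimeScore for dead-weight holders until time expires, otherwise the last remaining ball ends the game.
; Helpers destroy balls, find the closest ball or objective holder, and spawn the capture ball.
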(event Custom|ConstructTestBall
  (for _index (range 1 (Variables|Default|GetBallCount))
    (Class|GameplayStatics|CreatePlayer _index))
  (bind _outactors (Actor|GetAllActorsOfClass "/Game/BluePrints/BP_Spawn.BP_Spawn_C"))
  (for _index_2 (range 0 (Variables|Default|GetBallCount))
    (bind _ballspawnloc (Default|GetPinballSpawnLocation (Utilities|Array|Get(acopy) _outactors _index_2)))
    (bind _returnvalue (Game|SpawnActorfromClass "/Game/BluePrints/BP_TestBall.BP_TestBall_C" (Math|Transform|MakeTransform _ballspawnloc "0, 0, 0" "1,1,1") "Undefined" 0 _index_2 self 0))
    (Variables|/Game/BluePrints/BP_TestBall.BP_TestBall_C|SetSpawnPosition _returnvalue _ballspawnloc)
    (Utilities|Array|AddUnique (Variables|Default|GetTestBalls) _returnvalue)
    (Utilities|Array|Resize (Variables|OddBallMode|GetTimeScore) 4))
  (General|PossessPlayers))

(event EventTick
  (params (DeltaSeconds :type Float%20%28single-precision%29))
  (switch int (Variables|Default|GetMode)
    (:Default
      (PinBallMode|DetectEndGame :!label _label))
    (:0
      (goto _label))
    (:1
      (CallFunction|DetectOddBallEndGame)
      (for _array_element (Variables|Default|GetTestBalls)
        (if (Variables|/Game/BluePrints/BP_TestBall.BP_TestBall_C|GethasDeadWeight _array_element)
          (Utilities|Array|SetArrayElem (Variables|OddBallMode|GetTimeScore) (Variables|/Game/BluePrints/BP_TestBall.BP_TestBall_C|GetctrlID _array_element) (+ (Utilities|Array|Get(acopy) (Variables|OddBallMode|GetTimeScore) (Variables|/Game/BluePrints/BP_TestBall.BP_TestBall_C|GetctrlID _array_element)) (Utilities|Time|GetWorldDeltaSeconds))))))))

(fn ConstructionScript)

(fn GetBallCount
  (return (Utilities|Array|Length (Variables|Default|GetTestBalls))))

(fn DestoryBall
  (params (idx :type Integer))
  (bind _returnvalue (Game|Player|GetPlayerPawn idx))
  (bind _asbp_test_ball (Utilities|Casting|CastToBP_TestBall _returnvalue))
  (Utilities|Array|RemoveItem (Variables|Default|GetTestBalls) _asbp_test_ball)
  (Default|SetViewPort (.AsPC%20Ball (Utilities|Casting|CastToPC_Ball (Game|GetPlayerController (Variables|/Game/BluePrints/BP_TestBall.BP_TestBall_C|GetctrlID _asbp_test_ball)))))
  (Actor|DestroyActor _asbp_test_ball) ; Camera will be destroy if active this node
)

(fn ClearBalls
  (if (> (Utilities|Array|Length (Variables|Default|GetTestBalls)) 0)
    (Utilities|Array|Clear (Variables|Default|GetTestBalls))
    (return)
    (else
      (return))))

(fn DetectEndGame
  (bind _ballcount (General|GetBallCount))
  (if (== _ballcount 1)
    (bind _asgm_pin_ball (Utilities|Casting|CastToGM_PinBall (Game|GetGameMode)))
    (Default|EndGame _asgm_pin_ball)
    (Actor|DestroyActor)
    (else
      (return))))

(fn CalculateClosestBall
  (params (ballNeedsOther :type BP%20Test%20Ball%20Object%20Reference))
  (LocalVariables|SetBallThatNeedsOthers ballNeedsOther)
  (for (_array_element _array_index) (Variables|Default|GetTestBalls)
    (if (!= _array_element (LocalVariables|GetBallThatNeedsOthers))
      (if (< (Transformation|GetDistanceTo (LocalVariables|GetBallThatNeedsOthers) _array_element) (LocalVariables|GetclosestDistance))
        (LocalVariables|SetclosestDistance (Transformation|GetDistanceTo (LocalVariables|GetBallThatNeedsOthers) _array_element))
        (LocalVariables|SetindexOfClosestBall _array_index))))
  (return (Utilities|Array|Get(acopy) (Variables|Default|GetTestBalls) (LocalVariables|GetindexOfClosestBall))))

(fn PossessPlayers
  (for _array_element (Variables|Default|GetTestBalls)
    (Pawn|Possess (Game|GetPlayerController (Variables|/Game/BluePrints/BP_TestBall.BP_TestBall_C|GetctrlID _array_element)) _array_element)
    (Default|SetViewPort (.AsPC%20Ball (Utilities|Casting|CastToPC_Ball (Game|GetPlayerController (Variables|/Game/BluePrints/BP_TestBall.BP_TestBall_C|GetctrlID _array_element)))))))

(fn DetectOddBallEndGame
  (bind _returnvalue (Game|GetGameMode))
  (bind (_asgm_odd_ball _bsuccess) (Utilities|Casting|CastToGM_OddBall _returnvalue))
  (if (and _bsuccess (<= (Variables|/Game/BluePrints/GM_OddBall.GM_OddBall_C|GetGamePlayTime _asgm_odd_ball) 0.01))
    (Default|EndGame _asgm_odd_ball)
    (else
      (return))))

(fn CreateCaptureBall
  (bind _returnvalue (Game|SpawnActorfromClass "/Game/BluePrints/BP_CaptureBall.BP_CaptureBall_C" (Math|Transform|MakeTransform (Math|Vector|MakeVector 0.0 0.0 (Math|Random|RandomFloatinRange 2e+02 2.5e+02)) "0, 0, 0" "1,1,1") "Undefined" 0 self 0))
  (Variables|OddBallMode|SetCaptureBall _returnvalue))

(fn GetBallThatHasObjective
  (for _array_element (Variables|Default|GetTestBalls)
    (if (and (Variables|/Game/BluePrints/BP_TestBall.BP_TestBall_C|GethasDeadWeight _array_element) (>= (Variables|/Game/BluePrints/BP_TestBall.BP_TestBall_C|GetGrabbingTimer _array_element) 0.0))
      (LocalVariables|SettempBall _array_element)))
  (return (LocalVariables|GettempBall)))