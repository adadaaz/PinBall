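; Game mode for the lava ball game, running multiplayer rounds and handling pause, game over and quit.
; BeginPlay spawns BP_BallManager to build the balls; DetectEndGame triggers a round check once one or none remains.
; The check either rebuilds balls after a delay or pauses with GameOver widgets per player.
; HUD creation is disconnected, and separate BP_Pinball spawn and possess functions go uncalled here.
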(event Custom|Start%20Game
  (CallFunction|CreatePlayers)
  (CallFunction|ResetGame))

(event Custom|PauseGame
  (bind _returnvalue (Game|GetPlayerController 0))
  ;[1 1 1] Pause Game
  (Game|SetGamePaused true)
  (Utilities|IsValid (Variables|Default|GetPauseWindow)
    (:Is%20Valid
      _)
    (:Is%20Not%20Valid
      (bind _returnvalue_2 (UserInterface|CreateWidget "/Game/UI/Pause.Pause_C" (Game|GetPlayerController 0)))
      (Variables|Default|SetPauseWindow _returnvalue_2)))
  (UserInterface|Viewport|AddtoViewport (Variables|Default|GetPauseWindow) 0)
  (Variables|/Script/Engine.PlayerController|SetbShowMouseCursor _returnvalue true)
  (Input|SetInputModeUIOnly _returnvalue (Variables|Default|GetPauseWindow) "DoNotLock"))

(event Custom|EndGame
  ;[1 1 1] End Game
  (for _array_element (Variables|/Game/BluePrints/BP_BallManager.BP_BallManager_C|GetTestBalls (Variables|Default|GetBallGm))
    (bind _aspc_ball (Utilities|Casting|CastToPC_Ball (Game|GetPlayerController (Variables|/Game/BluePrints/BP_TestBall.BP_TestBall_C|GetctrlID _array_element))))
    (Viewport|RemoveAllWidgets)
    (Variables|/Script/Engine.PlayerController|SetbShowMouseCursor (Game|GetPlayerController (Variables|/Game/BluePrints/BP_TestBall.BP_TestBall_C|GetctrlID _array_element)) true)
    (bind _returnvalue (UserInterface|CreateWidget "/Game/UI/GameOver.GameOver_C" _aspc_ball))
    (UserInterface|Viewport|AddtoViewport _returnvalue 1)
    (Input|SetInputModeUIOnly (Game|GetPlayerController (Variables|/Game/BluePrints/BP_TestBall.BP_TestBall_C|GetctrlID _array_element)) _returnvalue "DoNotLock")
    (Game|SetGamePaused true)))

(event Custom|CreatePlayers
  ;[1 1 1] Create Balls
  (bind _returnvalue (Game|SpawnActorfromClass "/Game/BluePrints/BP_BallManager.BP_BallManager_C" (Math|Transform|MakeTransform "0, 0, 0" "0, 0, 0" "1,1,1") "DontSpawnIfColliding" 0 (- (Variables|Default|GetMaxPlayers) 1) 0 0))
  (bind _output_get (Variables|Default|SetBallGm _returnvalue))
  (Default|ConstructTestBall _output_get))

(event Custom|RoundsCheck
  ;[1 1 1] Check Round
  (if (== (Variables|Default|GetRounds) (- (Variables|Default|GetMaxRound) 1))
    (CallFunction|EndGame)
    (else
      (CallFunction|BeginRound))))

(event Custom|BeginRound
  (bind _ballgm (Variables|Default|GetBallGm))
  ;[1 1 1] Begin Round
  (Utilities|FlowControl|Delay 3.0)
  (bind _result (Math|Integer|IncrementInt (Variables|Default|GetRounds))
    (:%20%20
      (Development|PrintString (Utilities|String|Append "Round: " (Utilities|String|ToString(Integer) _result)) true true "(R=0.754928,G=1.000000,B=0.087961,A=1.000000)" 1e+01)
      (Default|ClearBalls _ballgm)
      (Default|ConstructTestBall _ballgm))))

(event Custom|Construct%20LevelSelector
  ;[1 1 1] Construct LevelSelector
  (Utilities|IsValid (Variables|Default|GetLevelSelector)
    (:Is%20Not%20Valid
      (bind _returnvalue (Game|SpawnActorfromClass "/Game/BluePrints/BP_LevelData.BP_LevelData_C" (Math|Transform|MakeTransform "0, 0, 0" "0, 0, 0" "1,1,1") "DontSpawnIfColliding" 0 0))
      (Variables|Default|SetLevelSelector _returnvalue))))

(event Custom|UnPauseGame
  (bind _returnvalue (Game|GetPlayerController 0))
  ;[1 1 1] Un Pause Game
  (Game|SetGamePaused false)
  (Viewport|RemoveAllWidgets)
  (UserInterface|Viewport|AddtoViewport (Variables|Default|GetmHUD) 0)
  (Variables|/Script/Engine.PlayerController|SetbShowMouseCursor _returnvalue false)
  (Input|SetInputModeGameOnly _returnvalue))

(event Custom|QuitGame
  ;[1 1 1] Quit Game
  (Game|QuitGame 0 "Quit"))

(event Custom|ResetGame
  (bind _returnvalue (Game|GetPlayerController 0))
  ;[1 1 1] Reset Game
  (Viewport|RemoveAllWidgets)
  (bind _aspc_ball (Utilities|Casting|CastToPC_Ball (Game|GetPlayerController 0)))
  (Variables|/Script/Engine.PlayerController|SetbShowMouseCursor _returnvalue false)
  (Input|SetInputModeGameOnly _returnvalue))

(event EventTick
  (params (DeltaSeconds :type Float%20%28single-precision%29))
  ;[1 1 1] Event Tick
)

(event EventBeginPlay
  ;[1 1 1] BeginPlay
  (CallFunction|StartGame)
  (Variables|Default|SetisLava true))

(fn ConstructionScript)

(fn GeneratePlayerCtrls
  (switch Utilities|FlowControl|Switch|SwitchonE_NumberOfPlayers (Variables|Default|GetNumOfPlayers)
    (:NewEnumerator0
      (bind _output_get (Variables|Default|SetMaxPlayers 2))
      (for _index (range 0 _output_get)
        (Class|GameplayStatics|CreatePlayer _index))
      (return))
    (:NewEnumerator1
      (bind _output_get_2 (Variables|Default|SetMaxPlayers 3))
      (for _index_2 (range 0 _output_get_2)
        (Class|GameplayStatics|CreatePlayer _index_2))
      (return))
    (:NewEnumerator2
      (bind _output_get_3 (Variables|Default|SetMaxPlayers 4))
      (for _index_3 (range 0 _output_get_3)
        (Class|GameplayStatics|CreatePlayer _index_3))
      (return))))

(fn CreateBall
  (params (NumOfBalls :type Integer))
  (if (> (Utilities|Array|Length (Variables|Default|GetBalls)) 0)
    (return)
    (else
      (CallFunction|GeneratePlayerCtrls)
      (bind _outactors (Actor|GetAllActorsOfClass "/Game/BluePrints/BP_Spawn.BP_Spawn_C"))
      (for _index (range 0 (- NumOfBalls 1))
        (bind _ballspawnloc (Default|GetPinballSpawnLocation (Utilities|Array|Get(acopy) _outactors _index)))
        (bind _returnvalue (Game|SpawnActorfromClass "/Game/BluePrints/BP_Pinball.BP_Pinball_C" (Math|Transform|MakeTransform _ballspawnloc "0, 0, 0" "1,1,1") "Undefined" 0 0 0 0))
        (Utilities|Array|AddUnique (Variables|Default|GetBalls) _returnvalue))
      (return))))

(fn PossesBalls
  (params (ball :type Array%20of%20BP%20Pinball%20Object%20References))
  (for (_array_element _array_index) ball
    (bind _output_get (Variables|/Game/BluePrints/BP_Pinball.BP_Pinball_C|SetCtrlId _array_element _array_index))
    (Development|PrintString (Utilities|String|ToString(Integer) _output_get))
    (Pawn|Possess (Game|GetPlayerController _output_get) _array_element)))

(fn DestoryBalls
  (bind _asbp_pinball (Utilities|Casting|CastToBP_Pinball (Game|Player|GetPlayerPawn (Variables|Default|GetCurrDestroyBallCtrlIndex))))
  (Utilities|Array|RemoveItem (Variables|Default|GetBalls) _asbp_pinball))

(fn DetectEndGame
  (if (> (Utilities|Array|Length (Variables|/Game/BluePrints/BP_BallManager.BP_BallManager_C|GetTestBalls (Variables|Default|GetBallGm))) 1)
    (return)
    (else
      (CallFunction|RoundsCheck))))