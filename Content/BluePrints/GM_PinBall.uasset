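; Game mode for the local multiplayer pinball arena, running match flow, pause and game-over screens.
; BeginPlay shows a startup image, finds the BP_Store, then spawns BP_BallManager to build player balls and creates the HUD.
; A delayed Tick periodically hands the HUD to each ball and clears spent power-up icons.
; Item events check the store or portal state per controller ID, while GeneratePlayerCtrls creates local players from the selected count.
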(event Custom|DiscardItem
  (params (Controller%20ID :type Integer))
  (bind _ballmg (Variables|Default|GetBallMG))
  (bind _testballs (Variables|/Game/BluePrints/BP_BallManager.BP_BallManager_C|GetTestBalls _ballmg))
  (bind _output (Utilities|Array|Get(acopy) _testballs Controller%20ID))
  ;[1 1 1] Discard Item ( Portal Ball )
  (if (Utilities|IsValid _output)
    (if (Variables|/Game/BluePrints/BP_TestBall.BP_TestBall_C|GetIsAbleToUsePortal _output)
      (Variables|/Game/BluePrints/BP_TestBall.BP_TestBall_C|SetIsAbleToUsePortal _output false)
      (Variables|/Game/BluePrints/BP_TestBall.BP_TestBall_C|SetItemActived _output true))))

(event Custom|PauseGame
  ;[1 1 1] Pause Game
  (if (not (Variables|/Game/BluePrints/BP_BallManager.BP_BallManager_C|GetGameEnded (Variables|Default|GetBallMG)))
    (Game|SetGamePaused true)
    (Utilities|IsValid (Variables|Default|GetPauseWindow)
      (:Is%20Valid
        _)
      (:Is%20Not%20Valid
        (bind _returnvalue (UserInterface|CreateWidget "/Game/UI/Pause.Pause_C" (Game|GetPlayerController 0)))
        (Variables|Default|SetPauseWindow _returnvalue)))
    (UserInterface|Viewport|AddtoViewport (Variables|Default|GetPauseWindow) 0)
    (Default|SetFocus (Variables|Default|GetPauseWindow))
    (Variables|/Script/Engine.PlayerController|SetbShowMouseCursor (Game|GetPlayerController 0) true)))

(event Custom|EndGame
  (bind _ballmg (Variables|Default|GetBallMG))
  (bind _testballs (Variables|/Game/BluePrints/BP_BallManager.BP_BallManager_C|GetTestBalls _ballmg))
  ;[1 1 1] End Game
  (Utilities|FlowControl|Delay 2.0)
  (if (> (Utilities|Array|Length _testballs) 0)
    (for _array_element _testballs
      (bind _aspc_ball (Utilities|Casting|CastToPC_Ball (Game|GetPlayerController (Variables|/Game/BluePrints/BP_TestBall.BP_TestBall_C|GetctrlID _array_element))))
      (Viewport|RemoveAllWidgets)
      (Variables|/Script/Engine.PlayerController|SetbShowMouseCursor (Game|GetPlayerController (Variables|/Game/BluePrints/BP_TestBall.BP_TestBall_C|GetctrlID _array_element)) false)
      (bind _returnvalue (UserInterface|CreateWidget "/Game/UI/ArenaGameover.ArenaGameover_C" _aspc_ball))
      (UserInterface|Viewport|AddtoViewport _returnvalue 1)
      (Pawn|UnPossess (Game|GetPlayerController (Variables|/Game/BluePrints/BP_TestBall.BP_TestBall_C|GetctrlID _array_element))))
    (else
      (Development|PrintString "More than 1 ball exists"))))

(event Custom|GetStore
  ;[1 1 1] Get Store
  (Utilities|IsValid (Variables|Default|GetStore)
    (:Is%20Not%20Valid
      (bind _outactors (Actor|GetAllActorsOfClass "/Game/BluePrints/Store/BP_Store.BP_Store_C"))
      (Variables|Default|SetStore (Utilities|Array|Get(acopy) _outactors)))))

(event Custom|StartGame
  ;[1 1 1] Start Game
  (CallFunction|CreatePlayers)
  (Variables|/Game/BluePrints/BP_BallManager.BP_BallManager_C|SetMode (Variables|Default|GetBallMG) 0)
  (CallFunction|ResetGame))

(event Custom|CreatePlayers
  ;[1 1 1] Create Balls
  (bind _returnvalue (Game|SpawnActorfromClass "/Game/BluePrints/BP_BallManager.BP_BallManager_C" (Math|Transform|MakeTransform "0, 0, 0" "0, 0, 0" "1,1,1") "DontSpawnIfColliding" 0 (- (Variables|Default|GetMaxPlayers) 1) 0 0))
  (bind _output_get (Variables|Default|SetBallMG _returnvalue))
  (Default|ConstructTestBall _output_get))

(event Custom|UpdateHUD
  ;[1 1 1] HUD Update
  (Utilities|IsValid (Variables|Default|GetmHUD)
    (:Is%20Valid
      (for _array_element (Variables|/Game/BluePrints/BP_BallManager.BP_BallManager_C|GetTestBalls (Variables|Default|GetBallMG))
        (Utilities|IsValid _array_element
          (:Is%20Valid
            (Variables|/Game/BluePrints/BP_TestBall.BP_TestBall_C|SetmHUD _array_element (Variables|Default|GetmHUD))))))
    (:Is%20Not%20Valid
      (Development|PrintText "\"Can't find HUD\"" true true "(R=1.000000,G=0.000000,B=0.200191,A=1.000000)"))))

(event Custom|UseItem
  (params (ControllerID :type Integer))
  (bind _ballmg (Variables|Default|GetBallMG))
  (bind _testballs (Variables|/Game/BluePrints/BP_BallManager.BP_BallManager_C|GetTestBalls _ballmg))
  (bind _output (Utilities|Array|Get(acopy) _testballs ControllerID))
  ;[1 1 1] Use Item
  (if (Utilities|IsValid (Utilities|Array|Get(acopy) (Variables|/Game/BluePrints/BP_BallManager.BP_BallManager_C|GetTestBalls (Variables|Default|GetBallMG)) ControllerID))
    (Game|Feedback|PlayDynamicForceFeedback (Game|GetPlayerController ControllerID) 0.2 0.1 true true true true)
    (bind (_canuse _avaliableitem) (Default|CanUseItem (Variables|Default|GetStore) ControllerID))
    (if (and _canuse (Utilities|Enum|NotEqual(Enum) (Variables|/Game/BluePrints/BP_TestBall.BP_TestBall_C|GetBallStatus _output) "NewEnumerator3"))
      (Variables|/Game/BluePrints/BP_TestBall.BP_TestBall_C|SetPurchasedItem _output _avaliableitem)
      (Default|ItemSelector _output))))

(event Custom|UnPauseGame
  (bind _returnvalue (Game|GetPlayerController 0))
  (bind _mhud (Variables|Default|GetmHUD))
  ;[1 1 1] Un Pause Game
  (Game|SetGamePaused false)
  (Viewport|RemoveAllWidgets)
  (if (Utilities|IsValid _mhud)
    (UserInterface|Viewport|AddtoViewport _mhud 0)
    (Variables|/Script/Engine.PlayerController|SetbShowMouseCursor _returnvalue false)
    (Input|SetInputModeGameOnly _returnvalue)))

(event Custom|QuitGame
  ;[1 1 1] Quit Game
  (Game|QuitGame 0 "Quit" false))

(event Custom|ResetGame
  (bind _returnvalue (Game|GetPlayerController 0))
  ;[1 1 1] Reset Game
  (bind _aspc_ball (Utilities|Casting|CastToPC_Ball (Game|GetPlayerController 0)))
  (Viewport|RemoveAllWidgets)
  (bind _returnvalue_2 (UserInterface|CreateWidget "/Game/UI/HUD.HUD_C" _aspc_ball))
  (bind _output_get (Variables|Default|SetmHUD _returnvalue_2))
  (Variables|/Game/UI/HUD.HUD_C|SetPlayerCount _output_get (- (Variables|Default|GetMaxPlayers) 1))
  (UserInterface|Viewport|AddtoViewport _returnvalue_2 0)
  (Variables|/Script/Engine.PlayerController|SetbShowMouseCursor _returnvalue false)
  (Input|SetInputModeGameOnly _returnvalue))

(event EventTick
  (params (DeltaSeconds :type Float%20%28single-precision%29))
  ;[1 1 1] Updates HUD
  (Utilities|FlowControl|Delay 3.0)
  (CallFunction|UpdateHUD)
  (CallFunction|RemovePowerUpIcon))

(event EventBeginPlay
  ;[1 1 1] BeginPlay
  (bind _returnvalue (UserInterface|CreateWidget "/Game/UI/StartupImage.StartupImage_C"))
  (UserInterface|Viewport|AddtoViewport _returnvalue 0)
  (Utilities|FlowControl|Delay 3.0)
  (CallFunction|GetStore)
  (CallFunction|StartGame))

(fn ConstructionScript)

(fn GeneratePlayerCtrls
  (switch Utilities|FlowControl|Switch|SwitchonE_NumberOfPlayers (Variables|Default|GetNumOfPlayers)
    (:NewEnumerator0
      (bind _output_get (Variables|Default|SetMaxPlayers 2))
      (for _index (range 0 _output_get)
        (Class|GameplayStatics|CreatePlayer _index))
      (return))
    (:NewEnumerator1
      (bind _output_get_2 (Variables|Default|SetMaxPlayers 3))
      (for _index_2 (range 0 _output_get_2)
        (Class|GameplayStatics|CreatePlayer _index_2))
      (return))
    (:NewEnumerator2
      (bind _output_get_3 (Variables|Default|SetMaxPlayers 4))
      (for _index_3 (range 0 _output_get_3)
        (Class|GameplayStatics|CreatePlayer _index_3))
      (return))))

(fn RemovePowerUpIcon
  (bind _array_element (Utilities|Array|ForEachLoopwithBreak (Variables|/Game/BluePrints/BP_BallManager.BP_BallManager_C|GetTestBalls (Variables|Default|GetBallMG)) :!label _label)
    (:LoopBody
      (if (Utilities|IsValid _array_element)
        (if (Variables|/Game/BluePrints/BP_TestBall.BP_TestBall_C|GetreadyDestroyPowerUp _array_element)
          (Default|RemovedUsedItem (Variables|Default|GetStore) (Variables|/Game/BluePrints/BP_TestBall.BP_TestBall_C|GetctrlID _array_element))
          (Variables|/Game/BluePrints/BP_TestBall.BP_TestBall_C|SetreadyDestroyPowerUp _array_element false)
          (Variables|/Game/BluePrints/BP_TestBall.BP_TestBall_C|SetItemActived _array_element false))
        (else
          (goto _label Break))))))