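; Breakable pickup shield that bounces BP_TestBall pinballs away horizontally until one breaks through.
; On hit, it pushes the ball, disables sphere collision if Health is under a dash-dependent threshold, and maps Health to a crack parameter on a dynamic material.
; An outer overlap records whether the ball is dashing; an inner overlap plays the break effect and destroys the shield.
; Health is only read here, never reduced.
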(event OnComponentBeginOverlap(InnerOverlap)
  (params (OverlappedComponent :type Primitive%20Component%20Object%20Reference) (OtherActor :type Actor%20Object%20Reference) (OtherComp :type Primitive%20Component%20Object%20Reference) (OtherBodyIndex :type Integer) (bFromSweep :type Boolean) (SweepResult :type Hit%20Result%20Structure%20%28by%20ref%29))
  ;[1 1 1] When the pinball breaks through
  (if (.bSuccess (Utilities|Casting|CastToBP_TestBall OtherActor))
    (Effects|SpawnEmitteratLocation "/Game/Particles_and_2D_Animation/Death_Energy/ShieldBreak_Energy.ShieldBreak_Energy" (Transformation|GetWorldLocation (Variables|Default|GetSphere)) "0, 0, 0" "5.000000,5.000000,5.000000")
    (Actor|DestroyActor)))

(event OnComponentBeginOverlap(OuterSphere)
  (params (OverlappedComponent :type Primitive%20Component%20Object%20Reference) (OtherActor :type Actor%20Object%20Reference) (OtherComp :type Primitive%20Component%20Object%20Reference) (OtherBodyIndex :type Integer) (bFromSweep :type Boolean) (SweepResult :type Hit%20Result%20Structure%20%28by%20ref%29))
  (bind (_asbp_test_ball _bsuccess) (Utilities|Casting|CastToBP_TestBall OtherActor))
  ;[1 1 1] See if other pinball is dashing or not
  (if _bsuccess
    (if (Variables|/Game/BluePrints/BP_TestBall.BP_TestBall_C|GetisDashing _asbp_test_ball)
      (Variables|Default|SetisCollidingPinballDashing true)
      (else
        (Variables|Default|SetisCollidingPinballDashing false)))))

(event EventBeginPlay
  (Variables|Default|SetstartingHealth (Variables|Default|Gethealth)))

(event Collision|EventHit
  (params (MyComp :type Primitive%20Component%20Object%20Reference) (Other :type Actor%20Object%20Reference) (OtherComp :type Primitive%20Component%20Object%20Reference) (bSelfMoved :type Boolean) (HitLocation :type Vector :default "0, 0, 0") (HitNormal :type Vector :default "0, 0, 0") (NormalImpulse :type Vector :default "0, 0, 0") (Hit :type Hit%20Result%20Structure%20%28by%20ref%29))
  (bind (_asbp_test_ball _bsuccess) (Utilities|Casting|CastToBP_TestBall Other))
  ;[1 1 1] When the shield gets hit
  (if _bsuccess
    (Variables|Default|SetcollidingPinball _asbp_test_ball)
    (Utilities|FlowControl|Sequence
      (:then_0
        ;[1 1 1] AddForce
        (bind _addforcedirection (CallFunction|CalcAddForceDirection))
        (Physics|AddForce (Variables|/Game/BluePrints/BP_TestBall.BP_TestBall_C|GetBall (Variables|Default|GetcollidingPinball)) (* _addforcedirection (Variables|Default|Getforce)) "None" true))
      (:then_1
        ;[1 1 1] See if the pinball can break through
        (if (Variables|Default|GetisCollidingPinballDashing)
          (if (<= (Variables|Default|Gethealth) 1.0)
            (Collision|SetCollisionEnabled (Variables|Default|GetSphere) "NoCollision"))
          (elif (<= (Variables|Default|Gethealth) 2.0)
            (Collision|SetCollisionEnabled (Variables|Default|GetSphere) "NoCollision"))))
      (:then_2
        (Rendering|Material|SetScalarParameterValue (Variables|Default|GetShieldMI) "Cracked" (Math|Float|MapRangeClamped (Variables|Default|Gethealth) (Variables|Default|GetstartingHealth) 1.0 0.0 1.0) :!class /Script/Engine.MaterialInstanceDynamic)))))

(fn ConstructionScript
  (bind _returnvalue (Rendering|Material|CreateDynamicMaterialInstance (Variables|Default|GetSphere) 0 "/Game/BluePrints/ItemSpawnPoint/Shield_MI.Shield_MI" "None" :!class /Script/Engine.PrimitiveComponent))
  (Variables|Default|SetShieldMI _returnvalue))

(fn CalcAddForceDirection
  (bind _returnvalue (Transformation|GetActorLocation))
  (bind _collidingpinball (Variables|Default|GetcollidingPinball))
  (bind _returnvalue_2 (Transformation|GetActorTransform _collidingpinball))
  (bind _returnvalue_3 (Math|Rotator|FindLookatRotation _returnvalue (.location _returnvalue_2)))
  (bind _returnvalue_4 (Math|Vector|GetForwardVector _returnvalue_3))
  (return (Math|Vector|MakeVector (.x _returnvalue_4) (.y _returnvalue_4) 0.0)))