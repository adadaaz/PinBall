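; Manager actor that spawns items at RandomItemSpawnPoint actors at random intervals.
; BeginPlay gathers every spawn point and picks a random index, using a range that leaves out the last array entry.
; Tick counts a timer down, then spawns at the chosen point and resets the timer between TimerMin and TimerMax.
; The index is rerolled only when that point already holds an item, retrying each frame.
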(event EventBeginPlay
  (bind _outactors (Actor|GetAllActorsOfClass "/Game/BluePrints/ItemSpawnPoint/RandomItemSpawnPoint.RandomItemSpawnPoint_C"))
  (for _array_element _outactors
    (Utilities|Array|AddUnique (Variables|Default|GetSpawnPoints) _array_element)
    (Variables|Default|SetRand (Math|Random|RandomInteger (- (Utilities|Array|Length (Variables|Default|GetSpawnPoints)) 1)))))

(event Collision|EventActorBeginOverlap
  (params (OtherActor :type Actor%20Object%20Reference)))

(event EventTick
  (params (DeltaSeconds :type Float%20%28single-precision%29))
  (bind _output_get (Variables|Default|SetTimer (- (Variables|Default|GetTimer) DeltaSeconds)))
  (Math|Float|CompareFloat _output_get 0.0
    (:<
      (bind _hasitem_ (Default|HasItem? (Utilities|Array|Get(acopy) (Variables|Default|GetSpawnPoints) (Variables|Default|GetRand))))
      (if _hasitem_
        (Variables|Default|SetRand (Math|Random|RandomInteger (- (Utilities|Array|Length (Variables|Default|GetSpawnPoints)) 1)))
        (else
          (Default|SpawnItem (Utilities|Array|Get(acopy) (Variables|Default|GetSpawnPoints) (Variables|Default|GetRand)))
          (Variables|Default|SetTimer (Math|Random|RandomFloatinRange (Variables|Default|GetTimerMin) (Variables|Default|GetTimerMax))))))))

(fn ConstructionScript)