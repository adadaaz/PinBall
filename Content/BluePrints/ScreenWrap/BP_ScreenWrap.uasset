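; Screen-wrap trigger volume that teleports an overlapping BP_TestBall pinball to the opposite side of the world origin.
; The trigger's dominant world axis (X or Y) picks which ball coordinate to negate, with a slight Z lift.
; The ball's HasScreenWrapped flag and cooldown guard against re-triggering, and a failed teleport retries once nudged inward.
; The construction script sizes the box from BoxExtent.
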(event OnComponentBeginOverlap(Box)
  (params (OverlappedComponent :type Primitive%20Component%20Object%20Reference) (OtherActor :type Actor%20Object%20Reference) (OtherComp :type Primitive%20Component%20Object%20Reference) (OtherBodyIndex :type Integer) (bFromSweep :type Boolean) (SweepResult :type Hit%20Result%20Structure%20%28by%20ref%29))
  (bind _defaultsceneroot (Variables|Default|GetDefaultSceneRoot))
  (bind _returnvalue (Transformation|GetWorldLocation _defaultsceneroot))
  (if (== (Utilities|GetClass OtherActor) "/Game/BluePrints/BP_TestBall.BP_TestBall_C")
    (bind _asbp_test_ball (Utilities|Casting|CastToBP_TestBall OtherActor))
    (bind _output_get (Variables|Default|Setpinball _asbp_test_ball))
    (if (not (Variables|/Game/BluePrints/BP_TestBall.BP_TestBall_C|GethasScreenWrapped _output_get))
      ;[1 1 1] Flip X on True, Flip Y on False
      (if (> (Math|Float|Absolute(Float) (.x _returnvalue)) (Math|Float|Absolute(Float) (.y _returnvalue)))
        ;[1 1 1] Teleport X
        (Variables|/Game/BluePrints/BP_TestBall.BP_TestBall_C|SethasScreenWrapped (Variables|Default|Getpinball) true)
        (Default|ScreenWrapCoolddown (Variables|Default|Getpinball))
        (bind _returnvalue_2 (Transformation|Teleport (Variables|Default|Getpinball) (Math|Vector|MakeVector (* (.x (Transformation|GetWorldLocation (Variables|/Game/BluePrints/BP_TestBall.BP_TestBall_C|GetBall (Variables|Default|Getpinball)))) -1.0) (.y (Transformation|GetWorldLocation (Variables|/Game/BluePrints/BP_TestBall.BP_TestBall_C|GetBall (Variables|Default|Getpinball)))) (+ (.z (Transformation|GetWorldLocation (Variables|/Game/BluePrints/BP_TestBall.BP_TestBall_C|GetBall (Variables|Default|Getpinball)))) 5e+01)) "0, 0, 0"))
        (if (not _returnvalue_2)
          (if (> (.x (Transformation|GetWorldLocation (Variables|/Game/BluePrints/BP_TestBall.BP_TestBall_C|GetBall (Variables|Default|Getpinball)))) 0.0)
            ;;[1 1 1] Try Again if failed
            (Transformation|Teleport (Variables|Default|Getpinball) (Math|Vector|MakeVector (+ (* (.x (Transformation|GetWorldLocation (Variables|/Game/BluePrints/BP_TestBall.BP_TestBall_C|GetBall (Variables|Default|Getpinball)))) -1.0) 2e+02) (.y (Transformation|GetWorldLocation (Variables|/Game/BluePrints/BP_TestBall.BP_TestBall_C|GetBall (Variables|Default|Getpinball)))) (+ (.z (Transformation|GetWorldLocation (Variables|/Game/BluePrints/BP_TestBall.BP_TestBall_C|GetBall (Variables|Default|Getpinball)))) 5e+01)) "0, 0, 0")
            (else
              (Transformation|Teleport (Variables|Default|Getpinball) (Math|Vector|MakeVector (+ (* (.x (Transformation|GetWorldLocation (Variables|/Game/BluePrints/BP_TestBall.BP_TestBall_C|GetBall (Variables|Default|Getpinball)))) -1.0) -2e+02) (.y (Transformation|GetWorldLocation (Variables|/Game/BluePrints/BP_TestBall.BP_TestBall_C|GetBall (Variables|Default|Getpinball)))) (+ (.z (Transformation|GetWorldLocation (Variables|/Game/BluePrints/BP_TestBall.BP_TestBall_C|GetBall (Variables|Default|Getpinball)))) 5e+01)) "0, 0, 0"))))
        (else
          ;[1 1 1] Teleport Y
          (Variables|/Game/BluePrints/BP_TestBall.BP_TestBall_C|SethasScreenWrapped (Variables|Default|Getpinball) true)
          (Default|ScreenWrapCoolddown (Variables|Default|Getpinball))
          (bind _returnvalue_3 (Transformation|Teleport (Variables|Default|Getpinball) (Math|Vector|MakeVector (.x (Transformation|GetWorldLocation (Variables|/Game/BluePrints/BP_TestBall.BP_TestBall_C|GetBall (Variables|Default|Getpinball)))) (* (.y (Transformation|GetWorldLocation (Variables|/Game/BluePrints/BP_TestBall.BP_TestBall_C|GetBall (Variables|Default|Getpinball)))) -1.0) (+ (.z (Transformation|GetWorldLocation (Variables|/Game/BluePrints/BP_TestBall.BP_TestBall_C|GetBall (Variables|Default|Getpinball)))) 5e+01)) "0, 0, 0"))
          (if (not _returnvalue_3)
            (if (> (.y (Transformation|GetWorldLocation (Variables|/Game/BluePrints/BP_TestBall.BP_TestBall_C|GetBall (Variables|Default|Getpinball)))) 0.0)
              ;;[1 1 1] Try Again if failed
              (Transformation|Teleport (Variables|Default|Getpinball) (Math|Vector|MakeVector (.x (Transformation|GetWorldLocation (Variables|/Game/BluePrints/BP_TestBall.BP_TestBall_C|GetBall (Variables|Default|Getpinball)))) (+ (* (.y (Transformation|GetWorldLocation (Variables|/Game/BluePrints/BP_TestBall.BP_TestBall_C|GetBall (Variables|Default|Getpinball)))) -1.0) 2e+02) (+ (.z (Transformation|GetWorldLocation (Variables|/Game/BluePrints/BP_TestBall.BP_TestBall_C|GetBall (Variables|Default|Getpinball)))) 5e+01)) "0, 0, 0")
              (else
                (Transformation|Teleport (Variables|Default|Getpinball) (Math|Vector|MakeVector (.x (Transformation|GetWorldLocation (Variables|/Game/BluePrints/BP_TestBall.BP_TestBall_C|GetBall (Variables|Default|Getpinball)))) (+ (* (.y (Transformation|GetWorldLocation (Variables|/Game/BluePrints/BP_TestBall.BP_TestBall_C|GetBall (Variables|Default|Getpinball)))) -1.0) -2e+02) (+ (.z (Transformation|GetWorldLocation (Variables|/Game/BluePrints/BP_TestBall.BP_TestBall_C|GetBall (Variables|Default|Getpinball)))) 5e+01)) "0, 0, 0")))))))))

(fn ConstructionScript
  (Components|Box|SetBoxExtent (Variables|Default|GetBox) (Variables|Default|GetboxExtent) true))