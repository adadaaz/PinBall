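; BP_HUDManager is an actor that owns the front-end menus: main menu, level select and game mode select.
; On BeginPlay it creates each widget once, adds all three to the viewport, sets UI-only input with a visible cursor, and shows the main menu.
; Display events switch screens by toggling visibility rather than recreating widgets.
; The level and game mode screens also set user focus on a default button.
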(event Custom|DisplayMainMenu
  (Widget|SetVisibility (Variables|Default|GetWG_LevelSelect) "Hidden")
  (Widget|SetVisibility (Variables|Default|GetWG_MainMenu) "Visible")
  (Widget|SetVisibility (Variables|Default|GetWG_GameModeSelect) "Hidden"))

(event Custom|DisplayGamemodeSelect
  (bind _wg_gamemodeselect (Variables|Default|GetWG_GameModeSelect))
  (Widget|SetVisibility (Variables|Default|GetWG_MainMenu) "Hidden")
  (Widget|SetVisibility (Variables|Default|GetWG_LevelSelect) "Hidden")
  (Widget|SetVisibility _wg_gamemodeselect "Visible")
  (Class|Widget|SetUserFocus (Variables|/Game/UI/GamemodeSelection.GamemodeSelection_C|Getbtn_infected _wg_gamemodeselect) (Game|GetPlayerController 0)))

(event Custom|DisplayLevelSelect
  (bind _wg_levelselect (Variables|Default|GetWG_LevelSelect))
  (Widget|SetVisibility (Variables|Default|GetWG_MainMenu) "Hidden")
  (Widget|SetVisibility _wg_levelselect "Visible")
  (Widget|SetVisibility (Variables|Default|GetWG_GameModeSelect) "Hidden")
  (Class|Widget|SetUserFocus (Variables|/Game/UI/Level/LevelSelect.LevelSelect_C|GetbtnMoreLeft _wg_levelselect) (Game|GetPlayerController 0)))

(event EventBeginPlay
  (CallFunction|CreateMainWidget)
  (CallFunction|CreateLevelWidget)
  (CallFunction|CreateGamemodeWidget)
  (CallFunction|DisplayMainMenu))

(event Collision|EventActorBeginOverlap
  (params (OtherActor :type Actor%20Object%20Reference)))

(event EventTick
  (params (DeltaSeconds :type Float%20%28single-precision%29)))

(fn ConstructionScript)

(fn CreateLevelWidget
  (bind _returnvalue (Game|GetPlayerController 0))
  (Utilities|IsValid (Variables|Default|GetWG_LevelSelect)
    (:Is%20Valid
      (return))
    (:Is%20Not%20Valid
      (bind _returnvalue_2 (UserInterface|CreateWidget "/Game/UI/Level/LevelSelect.LevelSelect_C" (Game|GetPlayerController 0)))
      (bind _output_get (Variables|Default|SetWG_LevelSelect _returnvalue_2))
      (Widget|SetVisibility _output_get "Hidden")
      (UserInterface|Viewport|AddtoViewport (Variables|Default|GetWG_LevelSelect) 0)
      (Variables|/Script/Engine.PlayerController|SetbShowMouseCursor _returnvalue true)
      (Input|SetInputModeUIOnly _returnvalue (Variables|Default|GetWG_LevelSelect) "DoNotLock"))))

(fn CreateMainWidget
  (bind _returnvalue (Game|GetPlayerController 0))
  (Utilities|IsValid (Variables|Default|GetWG_MainMenu)
    (:Is%20Valid
      (return))
    (:Is%20Not%20Valid
      (bind _returnvalue_2 (UserInterface|CreateWidget "/Game/UI/MainMenu.MainMenu_C" (Game|GetPlayerController 0)))
      (bind _output_get (Variables|Default|SetWG_MainMenu _returnvalue_2))
      (Widget|SetVisibility _output_get "Visible")
      (UserInterface|Viewport|AddtoViewport (Variables|Default|GetWG_MainMenu) 0)
      (Variables|/Script/Engine.PlayerController|SetbShowMouseCursor _returnvalue true)
      (Input|SetInputModeUIOnly _returnvalue (Variables|Default|GetWG_MainMenu) "DoNotLock")
      (Class|Widget|SetUserFocus (Variables|/Game/UI/MainMenu.MainMenu_C|GetbtnSettings _returnvalue_2) _returnvalue))))

(fn CreateGamemodeWidget
  (bind _returnvalue (Game|GetPlayerController 0))
  (Utilities|IsValid (Variables|Default|GetWG_GameModeSelect)
    (:Is%20Valid
      (return))
    (:Is%20Not%20Valid
      (bind _returnvalue_2 (UserInterface|CreateWidget "/Game/UI/GamemodeSelection.GamemodeSelection_C" (Game|GetPlayerController 0)))
      (bind _output_get (Variables|Default|SetWG_GameModeSelect _returnvalue_2))
      (Widget|SetVisibility _output_get "Hidden")
      (UserInterface|Viewport|AddtoViewport (Variables|Default|GetWG_GameModeSelect) 0)
      (Variables|/Script/Engine.PlayerController|SetbShowMouseCursor _returnvalue true)
      (Input|SetInputModeUIOnly _returnvalue (Variables|Default|GetWG_GameModeSelect) "DoNotLock"))))