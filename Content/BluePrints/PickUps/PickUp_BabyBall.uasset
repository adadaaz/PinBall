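; Baby Ball pickup that temporarily shrinks the player's physics ball, rotating each tick while in the level.
; Overlap with a PhysicsBallBP sets IsPickUp, hides the mesh and collision component, and makes both ignore the PhysicsBody channel instead of destroying the actor.
; It halves the ball's scale, then restores the saved scale after a ten-second delay, with debug prints around the wait.
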(event OnComponentBeginOverlap(PickUpCollision)
  (params (OverlappedComponent :type Primitive%20Component%20Object%20Reference) (OtherActor :type Actor%20Object%20Reference) (OtherComp :type Primitive%20Component%20Object%20Reference) (OtherBodyIndex :type Integer) (bFromSweep :type Boolean) (SweepResult :type Hit%20Result%20Structure%20%28by%20ref%29))
  ;[1 1 1] Baby Ball Collision
  (bind _asphysics_ball_bp (Utilities|Casting|CastToPhysicsBallBP OtherActor))
  (Variables|Default|SetIsPickUp true)
  (CallFunction|Impenetrable)
  (bind _output_get (Variables|Default|SetFormerScale (Transformation|GetActorScale3D _asphysics_ball_bp)))
  (Transformation|SetActorScale3D _asphysics_ball_bp (* _output_get "0.500000,0.500000,0.500000"))
  (Development|PrintString "Baby Ball Delay Begins" true true "(R=0.542126,G=0.510417,B=1.000000,A=1.000000)" 5.0)
  (Utilities|FlowControl|Delay 1e+01)
  (Development|PrintString "Baby Ball Delay Done" true true "(R=0.064768,G=0.000000,B=1.000000,A=1.000000)" 5.0)
  (Transformation|SetActorScale3D _asphysics_ball_bp (Variables|Default|GetFormerScale)))

(event Custom|Impenetrable
  (bind _babyballpickup (Variables|Default|GetBabyBallPickUp))
  ;[1 1 1] Makes pick up invisible & passible
  (Rendering|SetVisibility _babyballpickup false false)
  (Collision|SetCollisionResponsetoChannel _babyballpickup "ECC_PhysicsBody" "ECR_Ignore"))

(event EventBeginPlay)

(event Collision|EventActorBeginOverlap
  (params (OtherActor :type Actor%20Object%20Reference)))

(event EventTick
  (params (DeltaSeconds :type Float%20%28single-precision%29))
  ;[1 1 1] Rotates Pick-Up
  (Transformation|AddActorLocalRotation (Variables|Default|GetPickUpRotation) false false))

(fn ConstructionScript)