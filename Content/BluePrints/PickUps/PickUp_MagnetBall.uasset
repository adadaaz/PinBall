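; Magnet ball pickup actor that spins in place and grants the player ball the ability to use an item.
; Tick adds a local rotation each frame for the spin.
; When a BP_TestBall overlaps the collision component, it sets that ball's ItemAbleToUse flag, then hides the collision and magnet components and sets them to ignore the PhysicsBody channel instead of destroying the actor.
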(event OnComponentBeginOverlap(PickUpCollision)
  (params (OverlappedComponent :type Primitive%20Component%20Object%20Reference) (OtherActor :type Actor%20Object%20Reference) (OtherComp :type Primitive%20Component%20Object%20Reference) (OtherBodyIndex :type Integer) (bFromSweep :type Boolean) (SweepResult :type Hit%20Result%20Structure%20%28by%20ref%29))
  ;[1 1 1] Magnet Collision
  (bind _asbp_test_ball (Utilities|Casting|CastToBP_TestBall OtherActor))
  (Variables|/Game/BluePrints/BP_TestBall.BP_TestBall_C|SetItemAbleToUse _asbp_test_ball true)
  (CallFunction|Impenetrable))

(event Custom|Impenetrable
  (bind _pickupcollision (Variables|Default|GetPickUpCollision))
  ;[1 1 1] Makes pick up invisible & passible
  (Rendering|SetVisibility _pickupcollision false false)
  (Collision|SetCollisionResponsetoChannel _pickupcollision "ECC_PhysicsBody" "ECR_Ignore"))

(event EventBeginPlay)

(event Collision|EventActorBeginOverlap
  (params (OtherActor :type Actor%20Object%20Reference)))

(event EventTick
  (params (DeltaSeconds :type Float%20%28single-precision%29))
  ;[1 1 1] Rotates pick up
  (Transformation|AddActorLocalRotation (Variables|Default|GetPickUpRotation) false false))

(fn ConstructionScript)