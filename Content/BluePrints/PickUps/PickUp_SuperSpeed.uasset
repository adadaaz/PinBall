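; A rotating super-speed pickup that temporarily boosts the pinball player (BP_Pinball).
; On overlap it hides its collision component and visual, sets both to ignore the PhysicsBody channel, and multiplies the ball's max velocity and acceleration by 1.3.
; After a ten-second Delay it restores the saved values and clears its HasSuperSpeed flag.
; The pickup is never destroyed or re-enabled.
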(event OnComponentBeginOverlap(PickUpCollision)
  (params (OverlappedComponent :type Primitive%20Component%20Object%20Reference) (OtherActor :type Actor%20Object%20Reference) (OtherComp :type Primitive%20Component%20Object%20Reference) (OtherBodyIndex :type Integer) (bFromSweep :type Boolean) (SweepResult :type Hit%20Result%20Structure%20%28by%20ref%29))
  ;[1 1 1] Super Speed Collision
  (bind _asbp_pinball (Utilities|Casting|CastToBP_Pinball OtherActor))
  (Variables|Default|SethasSuperSpeed true)
  (CallFunction|Impenetrable)
  (bind _output_get (Variables|Default|SetFormerVelocity (Variables|/Game/BluePrints/BP_Pinball.BP_Pinball_C|GetMaxVelocity _asbp_pinball)))
  (bind _output_get_2 (Variables|Default|SetFormerAccel (Variables|/Game/BluePrints/BP_Pinball.BP_Pinball_C|GetPlayerAccel _asbp_pinball)))
  (Variables|/Game/BluePrints/BP_Pinball.BP_Pinball_C|SetMaxVelocity _asbp_pinball (* _output_get 1.3))
  (Variables|/Game/BluePrints/BP_Pinball.BP_Pinball_C|SetPlayerAccel _asbp_pinball (* _output_get_2 1.3))
  (Development|PrintString "Speed Delay Begins" true true "(R=0.542126,G=0.510417,B=1.000000,A=1.000000)" 5.0)
  (Utilities|FlowControl|Delay 1e+01)
  (Development|PrintString "Speed Delay Done" true true "(R=0.064768,G=0.000000,B=1.000000,A=1.000000)" 5.0)
  (Variables|/Game/BluePrints/BP_Pinball.BP_Pinball_C|SetMaxVelocity _asbp_pinball (Variables|Default|GetFormerVelocity))
  (Variables|/Game/BluePrints/BP_Pinball.BP_Pinball_C|SetPlayerAccel _asbp_pinball (Variables|Default|GetFormerAccel))
  (Variables|Default|SethasSuperSpeed false))

(event Custom|Impenetrable
  (bind _pickupcollision (Variables|Default|GetPickUpCollision))
  ;[1 1 1] Makes pick up invisible & passible
  (Rendering|SetVisibility _pickupcollision false false)
  (Collision|SetCollisionResponsetoChannel _pickupcollision "ECC_PhysicsBody" "ECR_Ignore"))

(event EventBeginPlay)

(event Collision|EventActorBeginOverlap
  (params (OtherActor :type Actor%20Object%20Reference)))

(event EventTick
  (params (DeltaSeconds :type Float%20%28single-precision%29))
  ;[1 1 1] Rotates pick up
  (Transformation|AddActorLocalRotation (Variables|Default|GetPickUpRotation) false false))

(fn ConstructionScript)