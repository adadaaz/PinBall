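; Base pickup actor that gives a ball (BP_TestBall) a power-up when the ball overlaps it.
; A ball without a power-up is flagged, and the DB_ItemList row for the pickup's name is written to BP_Store's waiting-item slot for its controller ID.
; The pickup then destroys itself, removes the store's first list item and clears its spawned flag.
; Balls already holding a power-up do not collect it.
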(event OnComponentBeginOverlap(Collision)
  (params (OverlappedComponent :type Primitive%20Component%20Object%20Reference) (OtherActor :type Actor%20Object%20Reference) (OtherComp :type Primitive%20Component%20Object%20Reference) (OtherBodyIndex :type Integer) (bFromSweep :type Boolean) (SweepResult :type Hit%20Result%20Structure%20%28by%20ref%29))
  (bind _storeref (Variables|Default|GetStoreRef))
  ;[1 1 1] Ball Collision
  (bind _asbp_test_ball (Utilities|Casting|CastToBP_TestBall OtherActor))
  (if (Variables|/Game/BluePrints/BP_TestBall.BP_TestBall_C|GethasPowerUp _asbp_test_ball)
    (Collision|SetCollisionResponsetoChannel (Variables|Default|GetCollision) "ECC_PhysicsBody" "ECR_Overlap")
    (else
      (CallFunction|Impenetrable)
      (CallFunction|AddtoStore (Variables|/Game/BluePrints/BP_TestBall.BP_TestBall_C|GetctrlID _asbp_test_ball))
      (Actor|DestroyActor)
      (Utilities|Array|RemoveIndex (Variables|/Game/BluePrints/Store/BP_Store.BP_Store_C|GetmItemList _storeref))
      (Variables|/Game/BluePrints/Store/BP_Store.BP_Store_C|SetSpawned _storeref false))))

(event Custom|Impenetrable
  (bind _pickupshape (Variables|Default|GetPickUpShape))
  ;[1 1 1] Makes pick up invisible & passible
  (Rendering|SetVisibility _pickupshape false false)
  (Collision|SetCollisionResponsetoChannel _pickupshape "ECC_PhysicsBody" "ECR_Ignore"))

(event EventBeginPlay
  (Utilities|IsValid (Variables|Default|GetStoreRef)
    (:Is%20Not%20Valid
      (bind _outactors (Actor|GetAllActorsOfClass "/Game/BluePrints/Store/BP_Store.BP_Store_C"))
      (Variables|Default|SetStoreRef (Utilities|Array|Get(acopy) _outactors)))))

(fn ConstructionScript)

(fn AddtoStore
  (params (id :type Integer))
  (bind _asbp_test_ball (Utilities|Casting|CastToBP_TestBall (Game|Player|GetPlayerPawn id)))
  (Variables|/Game/BluePrints/BP_TestBall.BP_TestBall_C|SethasPowerUp _asbp_test_ball true)
  (bind _returnvalue (Utilities|GetDataTableRow "/Game/BluePrints/Store/DB_ItemList.DB_ItemList" (Variables|Default|GetPickUpName))
    (:then
      (Utilities|Array|SetArrayElem (Variables|/Game/BluePrints/Store/BP_Store.BP_Store_C|GetItemWaitForUsage (Variables|Default|GetStoreRef)) id _returnvalue)
      (Variables|/Game/BluePrints/Store/BP_Store.BP_Store_C|SetBuyerID (Variables|Default|GetStoreRef) id))))