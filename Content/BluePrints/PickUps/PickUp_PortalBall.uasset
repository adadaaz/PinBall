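; Rotating portal pickup that lets the pinball use a portal.
; When a BP_Pinball overlaps the collision component, it stores the ball's current world location as the pinball's portal location and enables portal use.
; It then counts as picked up, hiding its mesh and collision components and ignoring the PhysicsBody channel rather than being destroyed.
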(event OnComponentBeginOverlap(PickUpCollision)
  (params (OverlappedComponent :type Primitive%20Component%20Object%20Reference) (OtherActor :type Actor%20Object%20Reference) (OtherComp :type Primitive%20Component%20Object%20Reference) (OtherBodyIndex :type Integer) (bFromSweep :type Boolean) (SweepResult :type Hit%20Result%20Structure%20%28by%20ref%29))
  ;[1 1 1] Portal Collision
  (bind _asbp_pinball (Utilities|Casting|CastToBP_Pinball OtherActor))
  (Variables|Default|SetIsPickUp true)
  (CallFunction|Impenetrable)
  (Variables|/Game/BluePrints/BP_Pinball.BP_Pinball_C|SetPortalLocation _asbp_pinball (Transformation|GetWorldLocation (Variables|/Game/BluePrints/BP_Pinball.BP_Pinball_C|GetBall _asbp_pinball)))
  (Variables|/Game/BluePrints/BP_Pinball.BP_Pinball_C|SetIsAbleToUsePortal _asbp_pinball true))

(event Custom|Impenetrable
  (bind _pickupcollision (Variables|Default|GetPickUpCollision))
  ;[1 1 1] Makes pick up invisible & passible
  (Rendering|SetVisibility _pickupcollision false false)
  (Collision|SetCollisionResponsetoChannel _pickupcollision "ECC_PhysicsBody" "ECR_Ignore"))

(event EventBeginPlay)

(event Collision|EventActorBeginOverlap
  (params (OtherActor :type Actor%20Object%20Reference)))

(event EventTick
  (params (DeltaSeconds :type Float%20%28single-precision%29))
  ;[1 1 1] Rotates pick up
  (Transformation|AddActorLocalRotation (Variables|Default|GetPickUpRotation) false false))

(fn ConstructionScript)