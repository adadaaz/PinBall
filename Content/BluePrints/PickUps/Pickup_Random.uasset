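; Random pickup Blueprint that takes on one of four pickup identities each time it begins play.
; BeginPlay runs the parent logic, sets a yaw-only PickUpRotation, then rolls a random integer to set PickUpName to BabyBall, SuperSpeed, GrenadeBall or PortalBall.
; Tick and the construction script only call the parent, so any behavior that uses the name and rotation lives outside this Blueprint.
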(event EventBeginPlay
  (|CallParentFunction)
  (Variables|Default|SetPickUpRotation "0.000000,2.000000, 0")
  (switch int (Math|Random|RandomIntegerinRange 0 3)
    (:0
      (Variables|Default|SetPickUpName "BabyBall"))
    (:1
      (Variables|Default|SetPickUpName "SuperSpeed"))
    (:2
      (Variables|Default|SetPickUpName "GrenadeBall"))
    (:3
      (Variables|Default|SetPickUpName "PortalBall"))))

(event EventTick
  (params (DeltaSeconds :type Float%20%28single-precision%29))
  (|CallParentFunction DeltaSeconds))

(fn ConstructionScript
  (|CallParentFunction))