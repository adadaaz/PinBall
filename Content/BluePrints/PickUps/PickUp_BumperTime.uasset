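; Bumper Time pickup for the pinball game that spins in place and hands control of a bumper pawn to the player whose ball touches it.
; On overlap it hides itself, ignores physics bodies, spawns a Pawn_Bumper at its location and possesses it with that ball's player controller.
; A brief steam burst plays, then the ball respawns.
; Invisibility, invulnerability and flag-reset logic is left unconnected and never runs.
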(event OnComponentBeginOverlap(PickUpCollision)
  (params (OverlappedComponent :type Primitive%20Component%20Object%20Reference) (OtherActor :type Actor%20Object%20Reference) (OtherComp :type Primitive%20Component%20Object%20Reference) (OtherBodyIndex :type Integer) (bFromSweep :type Boolean) (SweepResult :type Hit%20Result%20Structure%20%28by%20ref%29))
  (bind _bumpertimepickup (Variables|Default|GetBumperTimePickUp))
  ;[1 1 1] Bumper Time Ball Collision
  (bind _asbp_pinball (Utilities|Casting|CastToBP_Pinball OtherActor))
  (Variables|Default|SethasBumperTime true)
  (Development|PrintString "PickedUp")
  (CallFunction|Impenetrable)
  (Transformation|SetWorldRotation _bumpertimepickup "0, 0, 0" false false)
  (Transformation|SetWorldScale3D _bumpertimepickup "1.000000,1.000000,1.000000")
  (bind _returnvalue (Game|SpawnActorfromClass "/Game/BluePrints/PickUps/Pawn_Bumper.Pawn_Bumper_C" (Transformation|GetWorldTransform _bumpertimepickup) "Undefined" 0 0))
  (Pawn|Possess (Game|GetPlayerController (Variables|/Game/BluePrints/BP_Pinball.BP_Pinball_C|GetCtrlId _asbp_pinball)) _returnvalue)
  (bind _returnvalue_2 (Effects|SpawnEmitteratLocation "/Game/StarterContent/Particles/P_Steam_Lit.P_Steam_Lit" (Transformation|GetActorLocation) "0, 0, 0" "7.000000,1.000000,7.000000"))
  (Utilities|FlowControl|Delay 0.5)
  (Components|DestroyComponent _returnvalue_2)
  (Default|Respawn _asbp_pinball))

(event Custom|Invulnerablility
  (params (OtherActor :type Actor%20Component%20Object%20Reference))
  ;[1 1 1] Makes the player invulnerable from hitting other players for 3 seconds
)

(event Custom|Impenetrable
  ;[1 1 1] Makes pick up invisible & passible
  (Rendering|SetVisibility (Variables|Default|GetPickUpCollision) false false)
  (Collision|SetCollisionResponsetoChannel (Variables|Default|GetBumperTimePickUp) "ECC_PhysicsBody" "ECR_Ignore"))

(event Custom|BriefInvisible
  (params (OtherActor :type Actor%20Component%20Object%20Reference))
  ;[1 1 1] Respawn
)

(event EventTick
  (params (DeltaSeconds :type Float%20%28single-precision%29))
  ;[1 1 1] Rotates pick up
  (Transformation|AddActorLocalRotation (Variables|Default|GetPickUpRotation) false false))

(fn ConstructionScript)