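; Pickup Blueprint that grants the player's physics ball the grenade explosion ability.
; It spins by adding a local rotation every tick.
; When a PhysicsBallBP overlaps the collision component, it sets that ball's HasExplosion flag and prints debug messages.
; The Impenetrable event then hides the collision and mesh components and sets them to ignore the PhysicsBody channel, rather than destroying the actor.
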(event OnComponentBeginOverlap(PickUpCollision)
  (params (OverlappedComponent :type Primitive%20Component%20Object%20Reference) (OtherActor :type Actor%20Object%20Reference) (OtherComp :type Primitive%20Component%20Object%20Reference) (OtherBodyIndex :type Integer) (bFromSweep :type Boolean) (SweepResult :type Hit%20Result%20Structure%20%28by%20ref%29))
  ;[1 1 1] Grenade Ball Collision
  (bind _asphysics_ball_bp (Utilities|Casting|CastToPhysicsBallBP OtherActor))
  (Variables|/Game/BluePrints/PhysicsBallBP.PhysicsBallBP_C|SethasExplosion _asphysics_ball_bp true)
  (Development|PrintString "PickedUp")
  (CallFunction|Impenetrable)
  (Development|PrintString "Explosion Began"))

(event Custom|Impenetrable
  (bind _pickupcollision (Variables|Default|GetPickUpCollision))
  ;[1 1 1] Makes pick up invisible & passible
  (Rendering|SetVisibility _pickupcollision false false)
  (Collision|SetCollisionResponsetoChannel _pickupcollision "ECC_PhysicsBody" "ECR_Ignore"))

(event Collision|EventActorBeginOverlap
  (params (OtherActor :type Actor%20Object%20Reference)))

(event EventTick
  (params (DeltaSeconds :type Float%20%28single-precision%29))
  ;[1 1 1] Rotates pick up
  (Transformation|AddActorLocalRotation (Variables|Default|GetPickUpRotation) false false))

(fn ConstructionScript)