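; BP_Hole_Magnet is a capsule-shaped force zone that pushes pinballs along the direction of its Arrow component.
; Capsule overlap events add and remove BP_Pinball actors in the CollidingPinballs array.
; Each Tick turns off velocity limiting on those balls, with no restore on exit, and applies Force as a mass-independent acceleration.
; The construction script sizes the capsule from CapsuleRadius.
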(event OnComponentEndOverlap(MagnetCapsule)
  (params (OverlappedComponent :type Primitive%20Component%20Object%20Reference) (OtherActor :type Actor%20Object%20Reference) (OtherComp :type Primitive%20Component%20Object%20Reference) (OtherBodyIndex :type Integer))
  ;[1 1 1] Remove leaving Pinballs
  (bind _asbp_pinball (Utilities|Casting|CastToBP_Pinball OtherActor))
  (Utilities|Array|RemoveItem (Variables|Default|GetCollidingPinballs) _asbp_pinball))

(event OnComponentBeginOverlap(MagnetCapsule)
  (params (OverlappedComponent :type Primitive%20Component%20Object%20Reference) (OtherActor :type Actor%20Object%20Reference) (OtherComp :type Primitive%20Component%20Object%20Reference) (OtherBodyIndex :type Integer) (bFromSweep :type Boolean) (SweepResult :type Hit%20Result%20Structure%20%28by%20ref%29))
  ;[1 1 1] Populate Colliding pinballs
  (bind _asbp_pinball (Utilities|Casting|CastToBP_Pinball OtherActor))
  (Utilities|Array|Add (Variables|Default|GetCollidingPinballs) _asbp_pinball))

(event EventTick
  (params (DeltaSeconds :type Float%20%28single-precision%29))
  ;[1 1 1] Push All Pinballs within the Array
  (for _array_element (Variables|Default|GetCollidingPinballs)
    (Variables|/Game/BluePrints/BP_Pinball.BP_Pinball_C|SetLimitVelocity _array_element false)
    (Physics|AddForce (Variables|/Game/BluePrints/BP_Pinball.BP_Pinball_C|GetBall _array_element) (* (Math|Vector|GetForwardVector (Transformation|GetWorldRotation (Variables|Default|GetArrow))) (Variables|Default|GetForce)) "None" true)))

(event EventBeginPlay)

(fn ConstructionScript
  (Components|Capsule|SetCapsuleRadius (Variables|Default|GetMagnetCapsule) (Variables|Default|GetCapsuleRadius) true))