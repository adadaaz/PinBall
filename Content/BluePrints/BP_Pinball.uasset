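; Player-controlled physics pinball for up to four local players who ram each other for score, with health and lives.
; Input adds force under a velocity cap; dash briefly lifts it and auto-aims at a nearby opponent within a cone.
; On hits, the faster ball scores and knocks back the other, the slower loses health, with per-opponent cooldowns.
; Also handles respawn invulnerability, slow strips, portal and explosion powerups, and per-player materials.
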(event Custom|Invulnerable
  ;[1 1 1] Makes the player invulnerable from hitting other players for 3 seconds
  (Collision|SetCollisionResponsetoChannel (Variables|Default|GetBall) "ECC_PhysicsBody" "ECR_Ignore")
  (Development|PrintString "Collison Disabled" true true "(R=1.000000,G=0.019096,B=0.000000,A=1.000000)" 3.0)
  (Utilities|FlowControl|Delay 3.0)
  (Collision|SetCollisionResponsetoChannel (Variables|Default|GetBall) "ECC_PhysicsBody" "ECR_Block")
  (Development|PrintString "Collison Activated" true true "(R=0.000000,G=0.660000,B=1.000000,A=1.000000)" 3.0))

(event Custom|RemoveUnableToTakeDamageFromPinballs
  (params (Pinball%20To%20Remove :type BP%20Pinball%20Object%20Reference))
  (bind _ctrlid (Variables|BP_Pinball_C|GetCtrlId Pinball%20To%20Remove))
  ;[1 1 1] Remove Pinballs from an array of pinballs the player couldn't take health damage from
  (Utilities|FlowControl|Sequence
    (:then_0
      (if (== _ctrlid 0)
        (Utilities|FlowControl|Delay (Variables|PlayerVars|GetCollisionReduceHealthCooldown))
        (Utilities|Array|RemoveItem (Variables|PlayerVars|GetUnableToTakeDamageFromPinballs) Pinball%20To%20Remove)))
    (:then_1
      (if (== _ctrlid 1)
        (Utilities|FlowControl|Delay (Variables|PlayerVars|GetCollisionReduceHealthCooldown))
        (Utilities|Array|RemoveItem (Variables|PlayerVars|GetUnableToTakeDamageFromPinballs) Pinball%20To%20Remove)))
    (:then_2
      (if (== _ctrlid 2)
        (Utilities|FlowControl|Delay (Variables|PlayerVars|GetCollisionReduceHealthCooldown))
        (Utilities|Array|RemoveItem (Variables|PlayerVars|GetUnableToTakeDamageFromPinballs) Pinball%20To%20Remove)))
    (:then_3
      (if (== _ctrlid 3)
        (Utilities|FlowControl|Delay (Variables|PlayerVars|GetCollisionReduceHealthCooldown))
        (Utilities|Array|RemoveItem (Variables|PlayerVars|GetUnableToTakeDamageFromPinballs) Pinball%20To%20Remove)))))

(event Custom|Respawn
  ;[1 1 1] Respawn
  (Transformation|SetWorldLocation (Variables|Default|GetBall) (Variables|Default|GetinitPos) false false)
  (Physics|SetPhysicsLinearVelocity (Variables|Default|GetBall) (Math|Vector|MakeVector 0.0 0.0 0.0) false "None")
  (Input|DisableInput (Game|GetPlayerController (Variables|PlayerVars|GetCtrlId)))
  (Rendering|SetVisibility (Variables|Default|GetBall) false false)
  (Utilities|FlowControl|Delay 0.5)
  (Input|EnableInput (Game|GetPlayerController (Variables|PlayerVars|GetCtrlId)))
  (Rendering|SetVisibility (Variables|Default|GetBall) true false)
  (CallFunction|Invulnerable))

(event Custom|DisableLimitTemp
  ;[1 1 1] Disable Limit Temp
  (Variables|PlayerVars|SetLimitVelocity false)
  (Utilities|FlowControl|Delay 0.3)
  (Variables|PlayerVars|SetLimitVelocity true))

(event Custom|RemoveUnableToScoreAgainstPinballs
  (params (Pinball%20To%20Remove :type BP%20Pinball%20Object%20Reference))
  (bind _ctrlid (Variables|BP_Pinball_C|GetCtrlId Pinball%20To%20Remove))
  ;[1 1 1] Remove Pinballs from an array of pinballs the player couldn't score against
  (Utilities|FlowControl|Sequence
    (:then_0
      (if (== _ctrlid 0)
        (Utilities|FlowControl|Delay (Variables|PlayerVars|GetCollisionAddScoreCooldown))
        (Utilities|Array|RemoveItem (Variables|PlayerVars|GetUnableToScoreAgainstPinballs) Pinball%20To%20Remove)))
    (:then_1
      (if (== _ctrlid 1)
        (Utilities|FlowControl|Delay (Variables|PlayerVars|GetCollisionAddScoreCooldown))
        (Utilities|Array|RemoveItem (Variables|PlayerVars|GetUnableToScoreAgainstPinballs) Pinball%20To%20Remove)))
    (:then_2
      (if (== _ctrlid 2)
        (Utilities|FlowControl|Delay (Variables|PlayerVars|GetCollisionAddScoreCooldown))
        (Utilities|Array|RemoveItem (Variables|PlayerVars|GetUnableToScoreAgainstPinballs) Pinball%20To%20Remove)))
    (:then_3
      (if (== _ctrlid 3)
        (Utilities|FlowControl|Delay (Variables|PlayerVars|GetCollisionAddScoreCooldown))
        (Utilities|Array|RemoveItem (Variables|PlayerVars|GetUnableToScoreAgainstPinballs) Pinball%20To%20Remove)))))

(event Custom|TempDisableInput
  (params (TimeToWait :type Float%20%28single-precision%29))
  (bind _ctrlid (Variables|PlayerVars|GetCtrlId))
  (bind _returnvalue (Game|GetPlayerController _ctrlid))
  ;[1 1 1] Temporarily Disable Input
  (Input|DisableInput _returnvalue)
  (Utilities|FlowControl|Delay TimeToWait)
  (Input|EnableInput _returnvalue))

(event EventBeginPlay
  (bind _playerscale (Variables|PlayerVars|GetPlayerScale))
  ;[1 1 1] setting initial position(respawn position) of the ball
  (Utilities|FlowControl|Sequence
    (:then_0
      ;;[1 1 1] Set initial position and scale
      (bind _outactors (Actor|GetAllActorsOfClass "/Game/BluePrints/BP_Spawn.BP_Spawn_C"))
      (bind _ballspawnloc (Default|GetPinballSpawnLocation (Utilities|Array|Get(acopy) _outactors)))
      (Variables|Default|SetinitPos _ballspawnloc)
      (Transformation|SetRelativeScale3D (Variables|Default|GetBall) (Math|Vector|MakeVector _playerscale _playerscale _playerscale)))
    (:then_1
      ;;[1 1 1] Populate list of other players for Dash
      (Utilities|FlowControl|Delay 1.0)
      (bind _outactors_2 (Actor|GetAllActorsOfClass "BP_Pinball_C"))
      (for _array_element _outactors_2
        (if (!= self _array_element)
          (Utilities|Array|Add (Variables|Default|GetotherPlayers) _array_element))))
    (:then_2
      ;;[1 1 1] Pick player specific material
      (Utilities|FlowControl|Delay 1.0)
      (CallFunction|PickMaterial))
    (:then_3
      ;;[1 1 1] Set Starting Life
      (Variables|PlayerVars|SetStartingLife (Math|Conversions|ToFloat(Integer) (Variables|PlayerVars|GetLife))))
    (:then_4
      ;;[1 1 1] Set Starting Health
      (Variables|PlayerVars|SetStartingHealth (Math|Conversions|ToFloat(Integer) (Variables|PlayerVars|GetHealth))))))

(event EventTick
  (params (DeltaSeconds :type Float%20%28single-precision%29))
  (bind _returnvalue (Transformation|GetVelocity))
  (bind (_x _y) (Math|Vector|BreakVector _returnvalue))
  ;[1 1 1] Set current Velocity and Forward Vector and applies the Apply Max Velocity
  (Variables|Default|SetDeltaT DeltaSeconds)
  (Variables|PlayerVars|SetForwardVector (Math|Vector|Normalize (Transformation|GetVelocity)))
  (Variables|PlayerVars|SetVelocity (Math|Float|Sqrt (+ (Math|Float|Square _x) (Math|Float|Square _y))))
  (MovementFunc|ReducePlayerHeight)
  (if (Variables|PlayerVars|GetLimitVelocity)
    (MovementFunc|ApplyMaxVelocity)))

(event Collision|EventHit
  (params (MyComp :type Primitive%20Component%20Object%20Reference) (Other :type Actor%20Object%20Reference) (OtherComp :type Primitive%20Component%20Object%20Reference) (bSelfMoved :type Boolean) (HitLocation :type Vector :default "0, 0, 0") (HitNormal :type Vector :default "0, 0, 0") (NormalImpulse :type Vector :default "0, 0, 0") (Hit :type Hit%20Result%20Structure%20%28by%20ref%29))
  ;[1 1 1] Check if ball hits another ball
  (MovementFunc|AddBallForce Other))

(event Input|ActionEvents|InputActionExplosion
  (params (Key :type Key%20Structure))
  ;[1 1 1] GrenadeBall
  (:Pressed
    (if (Variables|PowerUpsandStrips|GethasExplosion)
      (Effects|SpawnEmitteratLocation "/Game/StarterContent/Particles/P_Explosion.P_Explosion" (Transformation|GetActorLocation) "0, 0, 0" "10.000000,1.000000,10.000000")
      (Game|SpawnActorfromClass "/Game/BluePrints/PickUps/Explosion.Explosion_C" (Transformation|GetWorldTransform (Variables|Default|GetBall)) "Undefined" 0 0)
      (Variables|PowerUpsandStrips|SethasExplosion false))))

(event Input|ActionEvents|InputActionDash
  (params (Key :type Key%20Structure))
  ;[1 1 1] Dash
  (:Pressed
    (if (Variables|PlayerVars|GetcanDash)
      (Variables|PlayerVars|SetcanDash false)
      (Rendering|Material|SetScalarParameterValue (Variables|PlayerVars|GetplayerMaterialInstance) "OverallDesaturation" 0.5 :!class /Script/Engine.MaterialInstanceDynamic)
      (Rendering|Material|SetScalarParameterValue (Variables|PlayerVars|GetplayerMaterialInstance) "Metal" 0.0 :!class /Script/Engine.MaterialInstanceDynamic)
      (Rendering|Material|SetScalarParameterValue (Variables|PlayerVars|GetplayerMaterialInstance) "Roughness" 0.0 :!class /Script/Engine.MaterialInstanceDynamic)
      (Variables|PlayerVars|SetLimitVelocity false)
      (DashFunc|SetDashRotation)
      (Physics|SetPhysicsLinearVelocity (Variables|Default|GetBall) (Math|Vector|MakeVector 0.0 0.0 0.0) false "None")
      (bind _closestplayer (DashFunc|GetClosestPlayer))
      (bind _dashvector (DashFunc|GetDashVector _closestplayer))
      (Physics|AddForce (Variables|Default|GetBall) (Math|Vector|MakeVector (.x (* _dashvector (Variables|PlayerVars|GetPlayerDashSpeed))) (.y (* _dashvector (Variables|PlayerVars|GetPlayerDashSpeed))) 0.0) "None" true)
      (Utilities|FlowControl|Delay (Variables|PlayerVars|GetlimitVelocityWait))
      (Variables|PlayerVars|SetLimitVelocity true)
      (Utilities|FlowControl|Delay (Variables|PlayerVars|GetDashDelay))
      (Variables|PlayerVars|SetcanDash true)
      (Rendering|Material|SetScalarParameterValue (Variables|PlayerVars|GetplayerMaterialInstance) "OverallDesaturation" 0.0 :!class /Script/Engine.MaterialInstanceDynamic)
      (Rendering|Material|SetScalarParameterValue (Variables|PlayerVars|GetplayerMaterialInstance) "Metal" 0.35 :!class /Script/Engine.MaterialInstanceDynamic)
      (Rendering|Material|SetScalarParameterValue (Variables|PlayerVars|GetplayerMaterialInstance) "Roughness" 0.1 :!class /Script/Engine.MaterialInstanceDynamic))))

(event Input|ActionEvents|InputActionActivatePortal
  (params (Key :type Key%20Structure))
  ;[1 1 1] PortalBall
  (:Pressed
    (if (Variables|PowerUpsandStrips|GetIsAbleToUsePortal)
      (Transformation|SetWorldLocation (Variables|Default|GetBall) (Variables|Default|GetPortalLocation) false false)
      (Variables|PowerUpsandStrips|SetIsAbleToUsePortal false))))

(event Input|AxisEvents|InputAxisMoveForward
  (params (AxisValue :type Float%20%28single-precision%29))
  (bind _playeraccel (Variables|PlayerVars|GetPlayerAccel))
  ;[1 1 1] Movement
  (Physics|AddForce (Variables|Default|GetBall) (Math|Vector|MakeVector (* _playeraccel AxisValue) (* (stale Input|AxisEvents|InputAxisMoveRight AxisValue) _playeraccel) 0.0) "None" true))

(event Input|AxisEvents|InputAxisMoveRight
  (params (AxisValue :type Float%20%28single-precision%29))
  (bind _playeraccel (Variables|PlayerVars|GetPlayerAccel))
  ;[1 1 1] Movement
  (Physics|AddForce (Variables|Default|GetBall) (Math|Vector|MakeVector (* _playeraccel (stale Input|AxisEvents|InputAxisMoveForward AxisValue)) (* AxisValue _playeraccel) 0.0) "None" true))

(fn ConstructionScript
  (bind _ball (Variables|Default|GetBall))
  (Utilities|FlowControl|Sequence
    (:then_0
      (if (== (Variables|PlayerVars|GetCtrlId) 0)
        (Rendering|Material|SetMaterial _ball 0 "/Game/Rolling/Materials/MI_PlayerBall1.MI_PlayerBall1")))
    (:then_1
      (if (== (Variables|PlayerVars|GetCtrlId) 1)
        (Rendering|Material|SetMaterial _ball 0 "/Game/Rolling/Materials/MI_PlayerBall2.MI_PlayerBall2")))
    (:then_2
      (if (== (Variables|PlayerVars|GetCtrlId) 2)
        (Rendering|Material|SetMaterial _ball 0 "/Game/Rolling/Materials/MI_PlayerBall3.MI_PlayerBall3")))
    (:then_3
      (if (== (Variables|PlayerVars|GetCtrlId) 3)
        (Rendering|Material|SetMaterial _ball 0 "/Game/Rolling/Materials/MI_PlayerBall4.MI_PlayerBall4")))))

(fn ApplyMaxVelocity
  (bind _returnvalue (Transformation|GetVelocity))
  (bind _maxvelocity (Variables|PlayerVars|GetMaxVelocity))
  (bind (_x _y) (Math|Vector|BreakVector _returnvalue))
  (bind (_x_2 _y_2) (Math|Vector|BreakVector _returnvalue))
  (bind _returnvalue_2 (Math|Vector|MakeVector _x _y 0.0))
  (bind _returnvalue_3 (Math|Vector|Normalize _returnvalue_2))
  (bind _returnvalue_4 (* _returnvalue_3 _maxvelocity))
  (if (> (Math|Float|Sqrt (+ (Math|Float|Square _x_2) (Math|Float|Square _y_2))) (Variables|PlayerVars|GetMaxVelocity))
    (Physics|SetPhysicsLinearVelocity (Variables|Default|GetBall) (Math|Vector|MakeVector (.x _returnvalue_4) (.y _returnvalue_4) 0.0) false "None")))

(fn AddBallForce
  (params (CollidingActor :type Actor%20Object%20Reference))
  (bind _forwardvector (Variables|PlayerVars|GetForwardVector))
  (bind _pinballhitamount (Variables|PlayerVars|GetpinballHitAmount))
  (bind _returnvalue (* _forwardvector _pinballhitamount))
  (bind (_x _y) (Math|Vector|BreakVector _returnvalue))
  (bind _asbp_pinball (Utilities|Casting|CastToBP_Pinball CollidingActor))
  (MovementFunc|SetHitAmount)
  (if (> (Variables|PlayerVars|GetVelocity) (Variables|BP_Pinball_C|GetVelocity _asbp_pinball))
    (Score|PinballWinstheCollision _asbp_pinball)
    (CallFunction|TempDisableInput _asbp_pinball (Variables|PlayerVars|GetdisableInputWait))
    (if (Variables|PowerUpsandStrips|GethasBouncyBall)
      (CallFunction|DisableLimitTemp _asbp_pinball))
    (Physics|SetPhysicsLinearVelocity (Variables|BP_Pinball_C|GetBall _asbp_pinball) (Math|Vector|MakeVector _x _y 0.0) false "None")
    (else
      (Health/LifeFunc|PinballLosestheCollision _asbp_pinball))))

(fn SetHitAmount
  (if (Variables|PowerUpsandStrips|GethasBouncyBall)
    (Variables|PlayerVars|SetpinballHitAmount (* (Variables|PlayerVars|GetVelocity) (Variables|PowerUpsandStrips|GetBouncyBallHitForce)))
    (else
      (Variables|PlayerVars|SetpinballHitAmount (Variables|PlayerVars|GetVelocity))))
  (return))

(fn GetClosestPlayer
  (for _array_element (Variables|Default|GetotherPlayers)
    (if (Utilities|IsValid _array_element)
      (if (< (Transformation|GetDistanceTo _array_element) (LocalVariables|GetclosestDistance))
        (LocalVariables|SetclosestDistance (Transformation|GetDistanceTo _array_element))
        (LocalVariables|SetclosestActor _array_element))))
  (return (LocalVariables|GetclosestActor)))

(fn GetDashVector
  (params (ClosestPlayer :type Actor%20Object%20Reference))
  (if (<= (Transformation|GetDistanceTo ClosestPlayer) (Variables|PlayerVars|GetDashDistance))
    (bind _output_get (LocalVariables|SetoutVector (Math|Vector|GetUnitDirection(Vector) (Transformation|GetActorLocation) (Transformation|GetActorLocation ClosestPlayer))))
    (if (<= (Math|Float|Absolute(Float) (- (Variables|PlayerVars|GetdashRotation) (.Yaw (Math|Rotator|BreakRotator (Math|Rotator|MakeRotfromX _output_get))))) (Variables|PlayerVars|GetDashAngleCone))
      _
      (else
        (LocalVariables|SetoutVector (Variables|PlayerVars|GetdashVector) :!label _label)))
    (else
      (goto _label)))
  (return (LocalVariables|GetoutVector)))

(fn PickMaterial
  (switch int (Variables|PlayerVars|GetCtrlId)
    (:0
      (LocalVariables|SettempPlayerMaterialInstance "/Game/Rolling/Materials/MI_PlayerBall1.MI_PlayerBall1"))
    (:1
      (LocalVariables|SettempPlayerMaterialInstance "/Game/Rolling/Materials/MI_PlayerBall2.MI_PlayerBall2"))
    (:2
      (LocalVariables|SettempPlayerMaterialInstance "/Game/Rolling/Materials/MI_PlayerBall3.MI_PlayerBall3"))
    (:3
      (LocalVariables|SettempPlayerMaterialInstance "/Game/Rolling/Materials/MI_PlayerBall4.MI_PlayerBall4")))
  (bind _returnvalue (Rendering|Material|CreateDynamicMaterialInstance (LocalVariables|GettempPlayerMaterialInstance) :!class /Script/Engine.KismetMaterialLibrary))
  (Variables|PlayerVars|SetplayerMaterialInstance _returnvalue)
  (Rendering|Material|SetMaterial (Variables|Default|GetBall) 0 (Variables|PlayerVars|GetplayerMaterialInstance)))

(fn SetDashRotation
  (Variables|PlayerVars|SetdashRotation (.Yaw (Math|Rotator|BreakRotator (Math|Rotator|MakeRotfromX (Transformation|GetComponentVelocity (Variables|Default|GetBall))))))
  (Variables|PlayerVars|SetdashVector (Math|Vector|Normalize (Transformation|GetVelocity))))

(fn ReducePlayerHeight
  (bind _ball (Variables|Default|GetBall))
  (if (> (.z (Transformation|GetWorldLocation _ball)) (Variables|PlayerVars|GetMaxPlayerHeight))
    (Physics|AddForce _ball "0, 0,-100.000000" "None" true))
  (return))

(fn EnterSlowStrip
  (params (Slow%20Amount :type Float%20%28single-precision%29))
  (Class|PrimitiveComponent|SetLinearDamping (Variables|Default|GetBall) Slow%20Amount))

(fn LeaveSlowStrip
  (params (Slow%20Time :type Float%20%28single-precision%29) (Slow%20Amount :type Float%20%28single-precision%29))
  (Utilities|Time|SetTimerbyFunctionName self "RemoveSlow" Slow%20Time)
  (Class|PrimitiveComponent|SetLinearDamping (Variables|Default|GetBall) Slow%20Amount))

(fn RemoveSlow
  (Class|PrimitiveComponent|SetLinearDamping (Variables|Default|GetBall) 0.0))

(fn AddPinballCollisionScore
  (Variables|PlayerVars|SetScore (+ (Variables|PlayerVars|GetScore) (Variables|PlayerVars|GetPinballCollisionScore)))
  (return))

(fn PinballWinstheCollision
  (params (CollidingPinball :type BP%20Pinball%20Object%20Reference))
  (bind _unabletoscoreagainstpinballs (Variables|PlayerVars|GetUnableToScoreAgainstPinballs))
  (if (> (Utilities|Array|Length _unabletoscoreagainstpinballs) 0)
    (for _array_element _unabletoscoreagainstpinballs
      (if (not (== _array_element CollidingPinball))
        (Utilities|Array|Add (Variables|PlayerVars|GetUnableToScoreAgainstPinballs) CollidingPinball)
        (Score|AddPinballCollisionScore)
        (CallFunction|RemoveUnabletoScoreAgainstPinballs CollidingPinball)))
    (else
      (Utilities|Array|Add (Variables|PlayerVars|GetUnableToScoreAgainstPinballs) CollidingPinball)
      (Score|AddPinballCollisionScore)
      (CallFunction|RemoveUnabletoScoreAgainstPinballs CollidingPinball))))

(fn ReduceHealth
  (params (Amount%20to%20Reduce%20Health :type Integer))
  (Variables|PlayerVars|SetHealth (- (Variables|PlayerVars|GetHealth) Amount%20to%20Reduce%20Health))
  (return))

(fn PinballLosestheCollision
  (params (Colliding%20Pinball :type BP%20Pinball%20Object%20Reference))
  (bind _unabletotakedamagefrompinballs (Variables|PlayerVars|GetUnableToTakeDamageFromPinballs))
  (if (> (Utilities|Array|Length _unabletotakedamagefrompinballs) 0)
    (for _array_element _unabletotakedamagefrompinballs
      (if (not (== _array_element Colliding%20Pinball))
        (Utilities|Array|Add (Variables|PlayerVars|GetUnableToTakeDamageFromPinballs) Colliding%20Pinball)
        (Health/LifeFunc|ReduceHealth 1)
        (CallFunction|RemoveUnabletoTakeDamagefromPinballs Colliding%20Pinball)
        (Health/LifeFunc|CheckifDead)))
    (else
      (Utilities|Array|Add (Variables|PlayerVars|GetUnableToTakeDamageFromPinballs) Colliding%20Pinball)
      (Health/LifeFunc|ReduceHealth 1)
      (CallFunction|RemoveUnabletoTakeDamagefromPinballs Colliding%20Pinball)
      (Health/LifeFunc|CheckifDead))))

(fn CheckifDead
  (if (<= (Variables|PlayerVars|GetHealth) 0)
    (Variables|PlayerVars|SetHealth (Math|Float|Truncate (Variables|PlayerVars|GetStartingHealth)))
    (bind _output_get (Variables|PlayerVars|SetLife (- (Variables|PlayerVars|GetLife) 1)))
    (if (> _output_get 0)
      (Health/LifeFunc|ResetVariablesonDeath)
      (CallFunction|Respawn)
      (else
        (Rendering|SetVisibility (Variables|Default|GetBall) false false)
        (bind _asgm_pin_ball (Utilities|Casting|CastToGM_PinBall (Game|GetGameMode)))
        (Variables|/Game/BluePrints/GM_PinBall.GM_PinBall_C|SetCurrDestroyBallCtrlIndex _asgm_pin_ball 0)
        (Default|DestoryBalls _asgm_pin_ball)))))

(fn ResetVariablesonDeath
  (Variables|PlayerVars|SetHealth (Math|Float|Truncate (Variables|PlayerVars|GetStartingHealth))))