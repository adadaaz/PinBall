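; BP_DeadZone is an overlap zone that takes one life from any BP_TestBall entering it.
; Balls with lives left respawn, except under the GM_Lavia game mode.
; At zero lives the ball is hidden; under GM_Lavia, BP_BallManager calculates player points from its controller ID.
; The zone writes those points and the death flag into the matching one of four game-mode player slots, then has the manager destroy the ball.
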(event EventBeginPlay)

(event Collision|EventActorBeginOverlap
  (params (OtherActor :type Actor%20Object%20Reference))
  (bind (_asbp_test_ball _bsuccess) (Utilities|Casting|CastToBP_TestBall OtherActor))
  (bind _ctrlid (Variables|/Game/BluePrints/BP_TestBall.BP_TestBall_C|GetctrlID _asbp_test_ball))
  (if _bsuccess
    (bind _output_get (Variables|/Game/BluePrints/BP_TestBall.BP_TestBall_C|SetCurrentLife _asbp_test_ball (- (Variables|/Game/BluePrints/BP_TestBall.BP_TestBall_C|GetCurrentLife _asbp_test_ball) 1)))
    (if (> _output_get 0)
      (if (not (.bSuccess (Utilities|Casting|CastToGM_Lavia (Game|GetGameMode))))
        (Default|Respawn _asbp_test_ball))
      (else
        (Rendering|SetVisibility (Variables|/Script/Engine.Actor|GetRootComponent _asbp_test_ball) false false)
        (bind _outactors (Actor|GetAllActorsOfClass "/Game/BluePrints/BP_BallManager.BP_BallManager_C"))
        (if (.bSuccess (Utilities|Casting|CastToGM_Lavia (Game|GetGameMode)))
          (Variables|Default|SetCtrlIdLava _ctrlid)
          (bind (_playerpoints _idplayers) (Default|CalculateOtherPlayerPoints (Utilities|Array|Get(acopy) _outactors) (Variables|Default|GetCtrlIdLava)))
          (Variables|Default|SetPlayerPointsRef _playerpoints)
          (Variables|Default|SetIDPlayersRef _idplayers)
          (Variables|Default|SetGM_LaviaRef (.AsGM%20Lavia (Utilities|Casting|CastToGM_Lavia (Game|GetGameMode))))
          (if (Utilities|Enum|Equal(Enum) _idplayers "0")
            (Variables|/Game/BluePrints/GM_Lavia.GM_Lavia_C|SetPlayer1Point (Variables|Default|GetGM_LaviaRef) (Variables|Default|GetPlayerPointsRef))
            (Variables|/Game/BluePrints/GM_Lavia.GM_Lavia_C|SetStringID (Variables|Default|GetGM_LaviaRef) "0")
            (Variables|/Game/BluePrints/GM_Lavia.GM_Lavia_C|SetIsDead1 (Variables|Default|GetGM_LaviaRef) true)
            (Default|DestoryBall (Utilities|Array|Get(acopy) _outactors) _ctrlid :!label _label)
            (elif (Utilities|Enum|Equal(Enum) (Variables|Default|GetIDPlayersRef) "1")
              (Variables|/Game/BluePrints/GM_Lavia.GM_Lavia_C|SetPlayer2Point (Variables|Default|GetGM_LaviaRef) (Variables|Default|GetPlayerPointsRef))
              (Variables|/Game/BluePrints/GM_Lavia.GM_Lavia_C|SetStringID (Variables|Default|GetGM_LaviaRef) "1")
              (Variables|/Game/BluePrints/GM_Lavia.GM_Lavia_C|SetIsDead2 (Variables|Default|GetGM_LaviaRef) true)
              (goto _label)
              (elif (Utilities|Enum|Equal(Enum) (Variables|Default|GetIDPlayersRef) "2")
                (Variables|/Game/BluePrints/GM_Lavia.GM_Lavia_C|SetPlayer3Point (Variables|Default|GetGM_LaviaRef) (Variables|Default|GetPlayerPointsRef))
                (Variables|/Game/BluePrints/GM_Lavia.GM_Lavia_C|SetStringID (Variables|Default|GetGM_LaviaRef) "2")
                (Variables|/Game/BluePrints/GM_Lavia.GM_Lavia_C|SetIsDead3 (Variables|Default|GetGM_LaviaRef) true)
                (goto _label)
                (elif (Utilities|Enum|Equal(Enum) (Variables|Default|GetIDPlayersRef) "3")
                  (Variables|/Game/BluePrints/GM_Lavia.GM_Lavia_C|SetPlayer4Point (Variables|Default|GetGM_LaviaRef) (Variables|Default|GetPlayerPointsRef))
                  (Variables|/Game/BluePrints/GM_Lavia.GM_Lavia_C|SetStringID (Variables|Default|GetGM_LaviaRef) "3")
                  (Variables|/Game/BluePrints/GM_Lavia.GM_Lavia_C|SetIsDead4 (Variables|Default|GetGM_LaviaRef) true)
                  (goto _label))))))))))

(fn ConstructionScript)