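; BP_Bumper_TronArena is a pinball bumper that awards score and knocks BP_TestBall away when hit.
; The hit pushes the ball horizontally away from the bumper's Arrow and plays a sound, light flare and scale pulse.
; Scoring locks for a cooldown, then randomly rolls whether the next hit pays the lottery score.
; A dynamic material instance on the mesh shows cooldown and lottery states.
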(event OnComponentHit(Bumper)
  (params (HitComponent :type Primitive%20Component%20Object%20Reference) (OtherActor :type Actor%20Object%20Reference) (OtherComp :type Primitive%20Component%20Object%20Reference) (NormalImpulse :type Vector :default "0, 0, 0") (Hit :type Hit%20Result%20Structure%20%28by%20ref%29))
  (bind (_asbp_test_ball _bsuccess) (Utilities|Casting|CastToBP_TestBall OtherActor))
  (if _bsuccess
    (Audio|SpawnSoundatLocation "/Game/Audio/Bumper_Cue.Bumper_Cue" "0, 0, 0" "0, 0, 0" 1.0 1.0 0.0 0 0)
    (Variables|Default|SetCollidingPinball _asbp_test_ball)
    (Variables|Default|SetBumperLocation (.location (Transformation|GetWorldTransform (Variables|Default|GetArrow))))
    (Utilities|FlowControl|Sequence
      (:then_0
        ;[1 1 1] Add Score
        (if (Variables|Default|GetGivesPoints)
          (Variables|Default|SetGivesPoints false)
          (Default|AddScore (Variables|Default|GetCollidingPinball) (Variables|Default|GetcurrentScoreWorth))
          (Rendering|Material|SetScalarParameterValue (Variables|Default|GetBumperMat) "isOnCooldown" 1.0 :!class /Script/Engine.MaterialInstanceDynamic)
          (Rendering|Material|SetScalarParameterValue (Variables|Default|GetBumperMat) "isLotteryBumper" 0.0 :!class /Script/Engine.MaterialInstanceDynamic)
          (Utilities|FlowControl|Delay (Variables|Default|GetCooldown))
          (Variables|Default|SetGivesPoints true)
          (Variables|Default|SetcurrentScoreWorth (Variables|Default|GetnormalScoreWorth))
          ;[1 1 1] Lottery Bumper
          (if (== (Math|Random|RandomIntegerinRange 1 (Variables|Default|GetlotteryChance)) (Variables|Default|GetlotteryChance))
            (Variables|Default|SetcurrentScoreWorth (Variables|Default|GetlotteryScoreWorth))
            (Rendering|Material|SetScalarParameterValue (Variables|Default|GetBumperMat) "isLotteryBumper" 1.0 :!class /Script/Engine.MaterialInstanceDynamic)
            (Audio|PlaySoundatLocation "/Game/Audio/Lottery_Bumper_Cue.Lottery_Bumper_Cue" "0, 0, 0" "0, 0, 0" 1.0 1.0 0.0 0 0 0)
            (else
              (Rendering|Material|SetScalarParameterValue (Variables|Default|GetBumperMat) "isOnCooldown" 0.0 :!class /Script/Engine.MaterialInstanceDynamic)))))
      (:then_1
        ;[1 1 1] Add Force
        (bind _addforcedirection (CallFunction|CalculateAddForceDirection))
        (bind _output_get (Variables|Default|SetAddForceDirection _addforcedirection))
        (Physics|AddForce (Variables|/Game/BluePrints/BP_TestBall.BP_TestBall_C|GetBall (Variables|Default|GetCollidingPinball)) (* _output_get (Variables|Default|GetForce)) "None" true))
      (:then_2
        ;[1 1 1] Pulse
        (if (not (Variables|Default|GetisPulsing))
          (Variables|Default|SetisPulsing true)
          (bind _intensity (Timeline|LightFlare PlayFromStart)
            (:Update
              (Rendering|Components|Light|SetIntensity (Variables|Default|GetPointLight) _intensity)
              (bind _size (Timeline|BumperPulse PlayFromStart)
                (:Update
                  (Transformation|SetRelativeScale3D (Variables|Default|GetPulse) _size))
                (:Finished
                  (Variables|Default|SetisPulsing false))))))))))

(event EventBeginPlay
  (Variables|Default|SetcurrentScoreWorth (Variables|Default|GetnormalScoreWorth)))

(fn ConstructionScript
  (bind _output_get (LocalVariables|SetTempMatInstance "/Game/Models/Infected/Materials/Bumper_Ring_MI.Bumper_Ring_MI"))
  (bind _returnvalue (Rendering|Material|CreateDynamicMaterialInstance _output_get "None" :!class /Script/Engine.KismetMaterialLibrary))
  (bind _output_get_2 (Variables|Default|SetBumperMat _returnvalue))
  (Rendering|Material|SetMaterial (Variables|Default|GetStaticMesh) 1 _output_get_2))

(fn CalculateAddForceDirection
  (bind _collidingpinball (Variables|Default|GetCollidingPinball))
  (bind _bumperlocation (Variables|Default|GetBumperLocation))
  (bind _returnvalue (Transformation|GetActorTransform _collidingpinball))
  (bind _returnvalue_2 (Math|Rotator|FindLookatRotation _bumperlocation (.location _returnvalue)))
  (bind _returnvalue_3 (Math|Vector|GetForwardVector _returnvalue_2))
  (return (Math|Vector|MakeVector (.x _returnvalue_3) (.y _returnvalue_3) 0.0)))