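; BP_Spawn is a per-player spawn point actor that provides a location for spawning a pinball.
; Its construction script uses PlayerID to read one of four player colors from the MPC_PlayerColor material parameter collection and tints the arrow component to match.
; GetPinballSpawnLocation converts the PinballLocation offset from the actor's local space into world space and returns it.
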(fn ConstructionScript
  (switch int (Variables|Default|GetPlayerID)
    (:0
      (bind _returnvalue (Rendering|Material|GetVectorParameterValue "/Game/Rolling/Materials/MPC_PlayerColor.MPC_PlayerColor" "Player1Color" :!class /Script/Engine.KismetMaterialLibrary))
      (LocalVariables|SetarrowColor _returnvalue))
    (:1
      (bind _returnvalue_2 (Rendering|Material|GetVectorParameterValue "/Game/Rolling/Materials/MPC_PlayerColor.MPC_PlayerColor" "Player2Color" :!class /Script/Engine.KismetMaterialLibrary))
      (LocalVariables|SetarrowColor _returnvalue_2))
    (:2
      (bind _returnvalue_3 (Rendering|Material|GetVectorParameterValue "/Game/Rolling/Materials/MPC_PlayerColor.MPC_PlayerColor" "Player3Color" :!class /Script/Engine.KismetMaterialLibrary))
      (LocalVariables|SetarrowColor _returnvalue_3))
    (:3
      (bind _returnvalue_4 (Rendering|Material|GetVectorParameterValue "/Game/Rolling/Materials/MPC_PlayerColor.MPC_PlayerColor" "Player4Color" :!class /Script/Engine.KismetMaterialLibrary))
      (LocalVariables|SetarrowColor _returnvalue_4)))
  (Variables|/Script/Engine.ArrowComponent|SetArrowColor (Variables|Default|GetArrow) (Math|Conversions|ToColor(LinearColor) (LocalVariables|GetarrowColor))))

(fn GetPinballSpawnLocation
  (return (Math|Transform|TransformLocation (Transformation|GetActorTransform) (Variables|Default|GetPinballLocation))))