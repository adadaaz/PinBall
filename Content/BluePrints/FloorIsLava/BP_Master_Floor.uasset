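; Master controller for a Floor Is Lava mode that picks floor pieces to shake and sink.
; On BeginPlay, WaveFunction sets a non-looping timer with a random delay that fires RunShake.
; RunShake picks a set number of random floors from FloorBlueprints, rebuilding the candidate list after each pick to avoid repeats.
; Each pick's ShakeFunction receives the shared shake, sink, stay-down and raise settings.
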(event EventBeginPlay
  (CallFunction|WaveFunction))

(fn ConstructionScript)

(fn WaveFunction
  (bind _returnvalue (Utilities|Time|SetTimerbyFunctionName 0 "RunShake" (Math|Random|RandomFloatinRange (Variables|Normal|GetminRandom) (Variables|Normal|GetmaxRandom))))
  (Variables|Default|SetWaveFunctionTimer _returnvalue))

(fn RunShake
  (for _array_element (Variables|Normal|GetfloorBlueprints)
    (Utilities|Array|Add (LocalVariables|GetlocalFloorsToSink) _array_element))
  (for _index (range 1 (Variables|Default|GetfloorsToSink))
    (LocalVariables|SetlocalCurrentIndex (Math|Random|RandomIntegerinRange 0 (- (Utilities|Array|Length (LocalVariables|GetlocalFloorsToSink)) 1)))
    (Default|ShakeFunction (Utilities|Array|Get(acopy) (LocalVariables|GetlocalFloorsToSink) (LocalVariables|GetlocalCurrentIndex)) (Variables|Normal|GetmaxShake) (Variables|Normal|GetdurationOfShake) (Variables|Normal|GettimeToStayDown) (Variables|Normal|GetsinkTime) (Variables|Normal|GetraiseTime))
    (Utilities|Array|Add (LocalVariables|GetlocalFloorsThatSank) (Utilities|Array|Get(acopy) (LocalVariables|GetlocalFloorsToSink) (LocalVariables|GetlocalCurrentIndex)))
    (Utilities|Array|Clear (LocalVariables|GetlocalFloorsToSink))
    (for _array_element_2 (Variables|Normal|GetfloorBlueprints)
      (if (== (Utilities|Array|FindItem (LocalVariables|GetlocalFloorsThatSank) _array_element_2) -1)
        (Utilities|Array|Add (LocalVariables|GetlocalFloorsToSink) _array_element_2)))))