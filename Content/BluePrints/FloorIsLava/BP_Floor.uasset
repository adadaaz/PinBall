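; Floor tile actor for a Floor Is Lava game that shakes with growing intensity when triggered through ShakeFunction.
; ShakeFunction stores the timing settings and arms Tick, which ramps shake amount over the duration and calls DoShake after short Delays.
; DoShake teleports the tile randomly along X and Y around its starting position, stopping at maximum shake.
; Sink, stay-down and raise times are stored, but no sinking or raising happens here.
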(event EventTick
  (params (DeltaSeconds :type Float%20%28single-precision%29))
  (if (Variables|Default|GetbeenCalled)
    (Variables|Default|SetSinkingSeconds (+ DeltaSeconds (Variables|Default|GetSinkingSeconds)))
    (if (and (> (Math|Float|MapRangeClamped (Variables|Default|GetSinkingSeconds) 0.0 (Variables|Default|GetdurationOfShake) 0.0 (Variables|Default|GetmaxShake)) 0.0) (<= (Math|Float|MapRangeClamped (Variables|Default|GetSinkingSeconds) 0.0 (Variables|Default|GetdurationOfShake) 0.0 (Variables|Default|GetmaxShake)) (Variables|Default|GetmaxShake)))
      (Utilities|FlowControl|Delay 0.05)
      (CallFunction|DoShake (Math|Float|MapRangeClamped (Variables|Default|GetSinkingSeconds) 0.0 (Variables|Default|GetdurationOfShake) 0.0 (Variables|Default|GetmaxShake))))))

(event EventBeginPlay
  (Variables|Default|SetstartingTransform (Transformation|GetActorTransform)))

(fn ConstructionScript
  (Components|StaticMesh|SetStaticMesh (Variables|Default|GetFloor) (Variables|Default|GetstaticMesh)))

(fn ShakeFunction
  (params (maxShake :type Float%20%28single-precision%29) (durationOfShake :type Float%20%28single-precision%29) (timeToStayDown :type Float%20%28single-precision%29) (sinkTime :type Float%20%28single-precision%29) (raiseTime :type Float%20%28single-precision%29))
  (CallFunction|SetVariables maxShake durationOfShake timeToStayDown sinkTime raiseTime)
  (Variables|Default|SetSinkingSeconds 0.0)
  (Variables|Default|SetbeenCalled true))

(fn SetVariables
  (params (maxShake :type Float%20%28single-precision%29) (durationOfShake :type Float%20%28single-precision%29) (timeToStayDown :type Float%20%28single-precision%29) (sinkTime :type Float%20%28single-precision%29) (raiseTime :type Float%20%28single-precision%29))
  (Variables|Default|SetmaxShake maxShake)
  (Variables|Default|SetdurationOfShake durationOfShake)
  (Variables|Default|SettimeToStayDown timeToStayDown)
  (Variables|Default|SetsinkTime sinkTime)
  (Variables|Default|SetraiseTime raiseTime)
  (return))

(fn DoShake
  (params (AmountToShake :type Float%20%28single-precision%29))
  (bind _returnvalue (Transformation|GetActorTransform))
  (bind _returnvalue_2 (Transformation|GetActorTransform))
  (bind _startingtransform (Variables|Default|GetstartingTransform))
  (bind _startingtransform_2 (Variables|Default|GetstartingTransform))
  (Utilities|FlowControl|Sequence
    (:then_0
      (switch int (Math|Random|RandomIntegerinRange 0 1)
        (:0
          (Transformation|SetActorRelativeTransform (Math|Transform|MakeTransform (Math|Vector|MakeVector (- (.x (.location _startingtransform)) AmountToShake) (.y (.location _startingtransform)) (.z (.location _startingtransform))) (.rotation _startingtransform) (.scale _startingtransform)) false true))
        (:1
          (Transformation|SetActorRelativeTransform (Math|Transform|MakeTransform (Math|Vector|MakeVector (+ (.x (.location _startingtransform_2)) AmountToShake) (.y (.location _startingtransform_2)) (.z (.location _startingtransform_2))) (.rotation _startingtransform_2) (.scale _startingtransform_2)) false true))))
    (:then_1
      (switch int (Math|Random|RandomIntegerinRange 0 1)
        (:0
          (Transformation|SetActorRelativeTransform (Math|Transform|MakeTransform (Math|Vector|MakeVector (.x (.location _returnvalue_2)) (- (.y (.location _returnvalue_2)) AmountToShake) (.z (.location _returnvalue_2))) (.rotation _returnvalue_2) (.scale _returnvalue_2)) false true))
        (:1
          (Transformation|SetActorRelativeTransform (Math|Transform|MakeTransform (Math|Vector|MakeVector (.x (.location _returnvalue)) (+ (.y (.location _returnvalue)) AmountToShake) (.z (.location _returnvalue))) (.rotation _returnvalue) (.scale _returnvalue)) false true))))
    (:then_2
      (if (>= AmountToShake (Variables|Default|GetmaxShake))
        (Variables|Default|SetbeenCalled false)
        (Development|PrintString "Finished Shake")))))