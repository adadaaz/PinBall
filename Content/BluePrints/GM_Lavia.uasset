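; Game mode for a round-based lava ball game that creates players, possesses them through the BallMG manager and sets the lava flag at start.
; Each tick checks for a single remaining ball and, while rounds remain, starts a delayed round that rebuilds test balls.
; EndGame pauses and shows a game-over widget per remaining ball's controller; ResetGame restores game-only input.
; HUD creation is unwired and UpdateHUD is empty.
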(event Custom|BeginRound
  (bind _ballmg (Variables|Default|GetBallMG))
  ;[1 1 1] BeginRound
  (Utilities|FlowControl|Delay 3.0)
  (bind _result (Math|Integer|IncrementInt (Variables|Default|GetRounds))
    (:%20%20
      (Development|PrintString (Utilities|String|Append "Round: " (Utilities|String|ToString(Integer) _result)) true true "(R=0.754928,G=1.000000,B=0.087961,A=1.000000)" 1e+01)
      (Utilities|Array|Clear (Variables|/Game/BluePrints/BP_BallManager.BP_BallManager_C|GetTestBalls _ballmg))
      (Default|ConstructTestBall _ballmg))))

(event Custom|StartLevel
  ;[1 1 1] StartLevel
  (CallFunction|CreatePlayers)
  (Default|PossessPlayer (Variables|Default|GetBallMG))
  (Variables|Default|SetisLava true))

(event Custom|ResetGame
  (bind _returnvalue (Game|GetPlayerController 0))
  ;[1 1 1] ResetGame
  (Viewport|RemoveAllWidgets)
  (Variables|/Script/Engine.PlayerController|SetbShowMouseCursor _returnvalue false)
  (Input|SetInputModeGameOnly _returnvalue))

(event Custom|CheckRounds
  ;[1 1 1] CheckRounds
  (bind _ballcount (Default|GetBallCount (Variables|Default|GetBallMG)))
  (if (and (== _ballcount 1) (< (Variables|Default|GetRounds) (- (Variables|Default|GetMaxRound) 1)))
    (CallFunction|BeginRound)))

(event Custom|EndGame
  ;[1 1 1] EndGame
  (for _array_element (Variables|/Game/BluePrints/BP_BallManager.BP_BallManager_C|GetBalls (Variables|Default|GetBallMG))
    (bind _aspc_ball (Utilities|Casting|CastToPC_Ball (Game|GetPlayerController (Variables|/Game/BluePrints/BP_Pinball.BP_Pinball_C|GetCtrlId _array_element))))
    (Viewport|RemoveAllWidgets)
    (Variables|/Script/Engine.PlayerController|SetbShowMouseCursor (Game|GetPlayerController (Variables|/Game/BluePrints/BP_Pinball.BP_Pinball_C|GetCtrlId _array_element)) true)
    (bind _returnvalue (UserInterface|CreateWidget "/Game/UI/GameOver.GameOver_C" _aspc_ball))
    (UserInterface|Viewport|AddtoViewport _returnvalue 1)
    (Input|SetInputModeUIOnly 0 _returnvalue "DoNotLock")
    (Game|SetGamePaused true)))

(event EventBeginPlay
  ;[1 1 1] BeginPlay
  (CallFunction|StartLevel))

(event EventTick
  (params (DeltaSeconds :type Float%20%28single-precision%29))
  ;[1 1 1] EventTick
  (CallFunction|CheckRounds))

(event EventUpdateHUD)

(fn ConstructionScript
  (|CallParentFunction))

(fn DetectEndGamee
  (if (> (Utilities|Array|Length (Variables|/Game/BluePrints/BP_BallManager.BP_BallManager_C|GetBalls (Variables|Default|GetBallMG))) 1)
    (return)
    (else
      (CallFunction|CheckRounds))))