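; BP_SlingShot is a slingshot bumper that launches a BP_TestBall on overlap, with sound and rumble.
; It zeroes the ball's velocity, then applies a velocity-change impulse along the capsule's forward vector, scaled by Force.
; Invert reverses the launch direction and mirrors the mesh in the construction script.
; An IsPulsing-guarded timeline drives light intensity and restarts a second scale-pulse timeline each update, whose finish clears the guard.
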(event Collision|EventActorBeginOverlap
  (params (OtherActor :type Actor%20Object%20Reference))
  (bind (_asbp_test_ball _bsuccess) (Utilities|Casting|CastToBP_TestBall OtherActor))
  (bind _ball (Variables|/Game/BluePrints/BP_TestBall.BP_TestBall_C|GetBall _asbp_test_ball))
  (if _bsuccess
    (Audio|PlaySoundatLocation "/Game/Audio/Slingshot_Cue.Slingshot_Cue" "0, 0, 0" "0, 0, 0" 1.0 1.0 0.0 0 0 0)
    (Default|PlayRumble _asbp_test_ball 0.5 0.15)
    (Physics|SetPhysicsLinearVelocity _ball "0, 0, 0" false "None")
    (if (Variables|Default|GetInvert)
      (Physics|AddImpulse _ball (* (Math|Vector|GetForwardVector (Variables|Default|GetCapsule)) (* (Variables|Default|GetForce) -1.0)) "None" true)
      (else
        (Physics|AddImpulse _ball (* (Math|Vector|GetForwardVector (Variables|Default|GetCapsule)) (Variables|Default|GetForce)) "None" true)))
    (if (not (Variables|Default|GetisPulsing))
      (Variables|Default|SetisPulsing true)
      (bind _intensity (Timeline|LightPusle PlayFromStart)
        (:Update
          (Rendering|Components|Light|SetIntensity (Variables|Default|GetPointLight) _intensity)
          (bind _pulse (Timeline|SizePulse PlayFromStart)
            (:Update
              (Transformation|SetRelativeScale3D (Variables|Default|Getpulse) (Math|Vector|MakeVector (.X (Math|Vector|BreakVector _pulse)) (.Y (Math|Vector|BreakVector _pulse)) 1.0)))
            (:Finished
              (Variables|Default|SetisPulsing false))))))))

(fn ConstructionScript
  (if (Variables|Default|GetInvert)
    (Transformation|SetRelativeScale3D (Variables|Default|GetStaticMesh) "-5.000000,5.000000,5.000000")))