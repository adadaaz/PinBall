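; Pinball bumper that awards score and pushes the ball away when hit.
; Points are gated by a cooldown, during which a dynamic material instance created in the construction script desaturates the bumper.
; Every hit, even during cooldown, applies a mass-independent force along the horizontal components of the direction from the Arrow component to the ball.
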(event OnComponentHit(Bumper)
  (params (HitComponent :type Primitive%20Component%20Object%20Reference) (OtherActor :type Actor%20Object%20Reference) (OtherComp :type Primitive%20Component%20Object%20Reference) (NormalImpulse :type Vector :default "0, 0, 0") (Hit :type Hit%20Result%20Structure%20%28by%20ref%29))
  (Variables|Default|SetCollidingPinball (.AsBP%20Test%20Ball (Utilities|Casting|CastToBP_TestBall OtherActor)))
  (Variables|Default|SetBumperLocation (.location (Transformation|GetWorldTransform (Variables|Default|GetArrow))))
  (Utilities|FlowControl|Sequence
    (:then_0
      ;[1 1 1] Add Score
      (if (Variables|Default|GetGivesPoints)
        (Variables|Default|SetGivesPoints false)
        (Default|AddScore (Variables|Default|GetCollidingPinball) (Variables|Default|GetScoreWorth))
        (Rendering|Material|SetScalarParameterValue (Variables|Default|GetBumperMat) "OverallDesaturation" 0.5 :!class /Script/Engine.MaterialInstanceDynamic)
        (Utilities|FlowControl|Delay (Variables|Default|GetCooldown))
        (Variables|Default|SetGivesPoints true)
        (Rendering|Material|SetScalarParameterValue (Variables|Default|GetBumperMat) "OverallDesaturation" 0.0 :!class /Script/Engine.MaterialInstanceDynamic)))
    (:then_1
      ;[1 1 1] Add Force
      (bind _addforcedirection (CallFunction|CalculateAddForceDirection))
      (bind _output_get (Variables|Default|SetAddForceDirection _addforcedirection))
      (Physics|AddForce (Variables|/Game/BluePrints/BP_TestBall.BP_TestBall_C|GetBall (Variables|Default|GetCollidingPinball)) (* _output_get (Variables|Default|GetForce)) "None" true))))

(fn ConstructionScript
  (bind _output_get (LocalVariables|SetTempMatInstance "/Game/Rolling/Materials/MI_Bumper.MI_Bumper"))
  (bind _returnvalue (Rendering|Material|CreateDynamicMaterialInstance _output_get "None" :!class /Script/Engine.KismetMaterialLibrary))
  (bind _output_get_2 (Variables|Default|SetBumperMat _returnvalue))
  (Rendering|Material|SetMaterial (Variables|Default|GetBumper) 0 _output_get_2))

(fn CalculateAddForceDirection
  (bind _collidingpinball (Variables|Default|GetCollidingPinball))
  (bind _bumperlocation (Variables|Default|GetBumperLocation))
  (bind _returnvalue (Transformation|GetActorTransform _collidingpinball))
  (bind _returnvalue_2 (Math|Rotator|FindLookatRotation _bumperlocation (.location _returnvalue)))
  (bind _returnvalue_3 (Math|Vector|GetForwardVector _returnvalue_2))
  (return (Math|Vector|MakeVector (.x _returnvalue_3) (.y _returnvalue_3) 0.0)))