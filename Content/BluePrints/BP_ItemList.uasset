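; BP_ItemList is a slot-based inventory that resizes its Slots array to MaxSize on BeginPlay.
; A slot counts as empty when its item class is invalid, and GetItemInfo reads an occupied slot's item data from class defaults.
; AddItem puts one item in the first empty slot and recurses for the remaining amount, so items never stack.
; It returns true once the first item fits, even if later ones do not.
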(event EventBeginPlay
  ;[1 1 1] Inventory System reference from: (https://www.youtube.com/watch?v=HjatBC6D1jc&list=PLmKKTERcjTPKEPl0nk48Tpmj-iWmzqo_Q&index=7
  (Utilities|Array|Resize (Variables|Default|GetSlots) (Variables|Default|GetMaxSize)))

(fn ConstructionScript)

(fn IsSlotEmpty?
  (params (index :type Integer))
  (return (not (Utilities|IsValidClass (.itemClass (Utilities|Struct|BreakS_PowerUpSlot (Utilities|Array|Get(acopy) (Variables|Default|GetSlots) index)))))))

(fn GetItemInfo
  (params (index :type Integer))
  (bind _slots (Variables|Default|GetSlots))
  (bind _output (Utilities|Array|Get(acopy) _slots index))
  (bind _itemclass (Utilities|Struct|BreakS_PowerUpSlot _output))
  (if (Utilities|IsValidClass _itemclass)
    (return false (Utilities|GetClassDefaults _itemclass))
    (else
      (return true ""))))

(fn SearchEmptySlot
  (bind (_array_element _array_index) (Utilities|Array|ForEachLoopwithBreak (Variables|Default|GetSlots) :!label _label)
    (:LoopBody
      (if (not (Utilities|IsValidClass (.itemClass (Utilities|Struct|BreakS_PowerUpSlot _array_element))))
        (LocalVariables|SetSearched true)
        (LocalVariables|SetlocalIndex _array_index)
        (goto _label Break)))
    (:Completed
      (return (LocalVariables|GetSearched) (LocalVariables|GetlocalIndex)))))

(fn AddItem
  (params (ItemClass :type BP%20Master%20Pickup%20Class%20Reference) (amount :type Integer))
  (LocalVariables|SetlocalClass ItemClass)
  (LocalVariables|SetlocalAmount amount)
  (bind (_success _index) (CallFunction|SearchEmptySlot))
  (if _success
    (bind _output_get (LocalVariables|SetavalibaleIndex _index))
    (Utilities|Array|SetArrayElem (Variables|Default|GetSlots) _output_get (Utilities|Struct|MakeS_PowerUpSlot (LocalVariables|GetlocalClass) 1))
    (if (> (LocalVariables|GetlocalAmount) 1)
      (CallFunction|AddItem (LocalVariables|GetlocalClass) (- (LocalVariables|GetlocalAmount) 1))
      (return true)
      (else
        (return true)))
    (else
      (return false))))