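; Game mode for the Infected minigame, a round-based infection contest between player balls scored by survival time.
; BeginPlay derives the round count from the player count and creates players, while Tick watches a flag to start rounds by infecting the next ball in turn.
; When CheckInfectedPlayers finds everyone infected, survival times are calculated and printed, then balls teleport to BP_Spawn points or the game pauses after the final round.
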(event Custom|EndGame
  ;[1 1 1] Game End
  (Game|SetGamePaused true)
  (CallFunction|CheckSurvivorsTime)
  (Development|PrintString "GameEnd"))

(event Custom|RoundStart
  ;[1 1 1] New Round Start
  (CallFunction|StartNewRound))

(event Custom|RoundEnd
  ;[1 1 1] Round End
  (for _array_element (Variables|/Game/BluePrints/BP_BallManager.BP_BallManager_C|GetTestBalls (Variables|Default|GetBallMG))
    (Default|CalculateSurvivalTime _array_element))
  (CallFunction|CheckSurvivorsTime)
  (CallFunction|CheckEndGame))

(event EventBeginPlay
  ;[1 1 1] BeginPlay
  (CallFunction|SetRound)
  (CallFunction|CreatePlayers)
  (Variables|/Game/BluePrints/BP_BallManager.BP_BallManager_C|SetMode (Variables|Default|GetBallMG) 2)
  (Viewport|RemoveAllWidgets)
  (Input|SetInputModeGameOnly (Game|GetPlayerController 0)))

(event EventTick
  (params (DeltaSeconds :type Float%20%28single-precision%29))
  ;[1 1 1] Checking New Rounds
  (if (Variables|Default|GetIsAbleToStartNewRound)
    (CallFunction|RoundStart)))

(fn ConstructionScript
  (|CallParentFunction))

(fn SetRound
  (switch Utilities|FlowControl|Switch|SwitchonE_NumberOfPlayers (Variables|Default|GetNumOfPlayers)
    (:NewEnumerator0
      (Variables|Default|SetGameRounds 1))
    (:NewEnumerator1
      (Variables|Default|SetGameRounds 2))
    (:NewEnumerator2
      (Variables|Default|SetGameRounds 3))))

(fn CheckInfectedPlayers
  (for _array_element (Variables|/Game/BluePrints/BP_BallManager.BP_BallManager_C|GetTestBalls (Variables|Default|GetBallMG))
    (if (not (Variables|/Game/BluePrints/BP_TestBall.BP_TestBall_C|GetIsInfected _array_element))
      (LocalVariables|SetAllInfected false)))
  (if (LocalVariables|GetAllInfected)
    (Development|PrintString "RoundEnd")
    (CallFunction|RoundEnd)))

(fn CheckSurvivorsTime
  (for (_array_element _array_index) (Variables|/Game/BluePrints/BP_BallManager.BP_BallManager_C|GetTestBalls (Variables|Default|GetBallMG))
    (Development|PrintString (Utilities|String|Append (Utilities|String|ToString(Integer) _array_index) (Utilities|String|ToString(Integer) (Math|Float|Floor (Variables|/Game/BluePrints/BP_TestBall.BP_TestBall_C|GetSurvivalTime _array_element)))) true true "(R=0.000000,G=0.660000,B=1.000000,A=1.000000)" 5e+01)))

(fn CheckEndGame
  (if (== (Variables|Default|GetGameRounds) (Variables|Default|GetInfectedPlayerIndex))
    (CallFunction|EndGame)
    (else
      (Variables|Default|SetInfectedPlayerIndex (+ (Variables|Default|GetInfectedPlayerIndex) 1))
      (Variables|Default|SetIsAbleToStartNewRound true)
      (bind _outactors (Actor|GetAllActorsOfClass "/Game/BluePrints/BP_Spawn.BP_Spawn_C"))
      (for _index (range 0 (Variables|Default|GetGameRounds))
        (bind _ballspawnloc (Default|GetPinballSpawnLocation (Utilities|Array|Get(acopy) _outactors _index)))
        (Transformation|SetWorldLocation (Variables|/Script/Engine.Actor|GetRootComponent (Utilities|Array|Get(acopy) (Variables|/Game/BluePrints/BP_BallManager.BP_BallManager_C|GetTestBalls (Variables|Default|GetBallMG)) _index)) _ballspawnloc false true)))))

(fn StartNewRound
  (Default|SetInfectedBall (Utilities|Array|Get(acopy) (Variables|/Game/BluePrints/BP_BallManager.BP_BallManager_C|GetTestBalls (Variables|Default|GetBallMG)) (Variables|Default|GetInfectedPlayerIndex)))
  (for _array_element (Variables|/Game/BluePrints/BP_BallManager.BP_BallManager_C|GetTestBalls (Variables|Default|GetBallMG))
    (Default|CheckDash _array_element))
  (Variables|Default|SetIsAbleToStartNewRound false))