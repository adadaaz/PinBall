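; BP_Ball_Spot_Light is a spotlight that follows a test ball and shows which controller it belongs to.
; On BeginPlay it sets the light color to one of four player colors based on the owning ball's CtrlID.
; Every Tick it rotates the SpotLight with a look-at rotation so it keeps pointing at that ball from the light's own location.
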(event EventTick
  (params (DeltaSeconds :type Float%20%28single-precision%29))
  (bind _spotlight (Variables|Default|GetSpotLight))
  (Transformation|SetWorldRotation _spotlight (Math|Rotator|FindLookatRotation (Transformation|GetWorldLocation _spotlight) (Transformation|GetActorLocation (Variables|Default|GetowningTestBall))) false false))

(event EventBeginPlay
  (bind _spotlight (Variables|Default|GetSpotLight))
  (switch int (Variables|/Game/BluePrints/BP_TestBall.BP_TestBall_C|GetctrlID (Variables|Default|GetowningTestBall))
    (:0
      (Rendering|Components|Light|SetLightColor _spotlight (Variables|Default|Getp1Color) true))
    (:1
      (Rendering|Components|Light|SetLightColor _spotlight (Variables|Default|Getp2Color) true))
    (:2
      (Rendering|Components|Light|SetLightColor _spotlight (Variables|Default|Getp3Color) true))
    (:3
      (Rendering|Components|Light|SetLightColor _spotlight (Variables|Default|Getp4Color) true))))

(fn ConstructionScript)