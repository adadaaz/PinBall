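; BP_SlingShot_Arena is an arena slingshot that launches a BP_TestBall when the ball overlaps it.
; On overlap it zeroes the ball's linear velocity, then applies a mass-independent impulse along the Capsule's forward vector, scaled by Force.
; The Invert flag reverses the launch direction, and the construction script mirrors the static mesh on X with a negative scale to match.
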(event Collision|EventActorBeginOverlap
  (params (OtherActor :type Actor%20Object%20Reference))
  (bind _asbp_test_ball (Utilities|Casting|CastToBP_TestBall OtherActor))
  (bind _ball (Variables|/Game/BluePrints/BP_TestBall.BP_TestBall_C|GetBall _asbp_test_ball))
  (Physics|SetPhysicsLinearVelocity _ball "0, 0, 0" false "None")
  (if (Variables|Default|GetInvert)
    (Physics|AddImpulse _ball (* (Math|Vector|GetForwardVector (Variables|Default|GetCapsule)) (* (Variables|Default|GetForce) -1.0)) "None" true)
    (else
      (Physics|AddImpulse _ball (* (Math|Vector|GetForwardVector (Variables|Default|GetCapsule)) (Variables|Default|GetForce)) "None" true))))

(fn ConstructionScript
  (if (Variables|Default|GetInvert)
    (Transformation|SetRelativeScale3D (Variables|Default|GetStaticMesh) "-5.000000,5.000000,5.000000")))