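; Slingshot bumper Blueprint for the arena that launches a BP_TestBall when it overlaps the actor.
; On overlap it plays a slingshot cue at the world origin, zeroes the ball's velocity, then applies a mass-independent impulse along the capsule's forward vector, scaled by Force.
; The Invert flag reverses that impulse, and the construction script uses it to mirror both static meshes through negative X scale and reposition the second.
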(event Collision|EventActorBeginOverlap
  (params (OtherActor :type Actor%20Object%20Reference))
  (bind _asbp_test_ball (Utilities|Casting|CastToBP_TestBall OtherActor))
  (bind _ball (Variables|/Game/BluePrints/BP_TestBall.BP_TestBall_C|GetBall _asbp_test_ball))
  (Audio|PlaySoundatLocation "/Game/Audio/Slingshot_Cue.Slingshot_Cue" "0, 0, 0" "0, 0, 0" 1.0 1.0 0.0 0 0 0)
  (Physics|SetPhysicsLinearVelocity _ball "0, 0, 0" false "None")
  (if (Variables|Default|GetInvert)
    (Physics|AddImpulse _ball (* (Math|Vector|GetForwardVector (Variables|Default|GetCapsule)) (* (Variables|Default|GetForce) -1.0)) "None" true)
    (else
      (Physics|AddImpulse _ball (* (Math|Vector|GetForwardVector (Variables|Default|GetCapsule)) (Variables|Default|GetForce)) "None" true))))

(fn ConstructionScript
  (bind _staticmesh1 (Variables|Default|GetStaticMesh1))
  (if (Variables|Default|GetInvert)
    (Transformation|SetRelativeScale3D (Variables|Default|GetStaticMesh) "-5.000000,5.000000,5.000000")
    (Transformation|SetRelativeScale3D _staticmesh1 "-175.000000,175.000000,175.000000")
    (Transformation|SetRelativeRotation _staticmesh1 "0,-80.000000, 0" false false)
    (Transformation|SetRelativeLocation _staticmesh1 "-48.000000,-10.000000,140.000000" false false)))